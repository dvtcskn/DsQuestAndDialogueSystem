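; Interactable NPC character for the quest and dialogue system that starts conversations with the player.
; BeginPlay sets its NPC interactable component and spawns a default controller if none exists.
; Its name and dialogue come from a data table row handle, with itself added as the NPC reference.
; Interact and EndInteract open and close the conversation through the NPCDialogueManager on the player's controller.
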(event `self.ReceiveBeginPlay`
  (set `self.Interactable` (`self.NPC_Interactable`))
  (`/Engine/EditorBlueprintResources/StandardMacros.IsValid` (`self.GetController`)
    (:`Is Not Valid`
      (`self.SpawnDefaultController`))))

(fn `EndInteract`
  (params (InCharacter :type "Character Object Reference"))
  (`parent.EndInteract` InCharacter)
  (bind _asbp_player_character (cast `/Game/SOsQuestAndDialogueSystem/Framework/Blueprints/BP_PlayerCharacter` InCharacter))
  (`/Game/SOsQuestAndDialogueSystem/Blueprints/DialogueSystem/BP_SOsDialogueManager_Component.EndCoversation` (`/Game/SOsQuestAndDialogueSystem/Framework/Blueprints/BP_TopDownController.NPCDialogueManager` (`/Game/SOsQuestAndDialogueSystem/Framework/Blueprints/BP_PlayerCharacter.GetPlayerControllerBP` _asbp_player_character))))

(fn `GetName`
  (returns (Return :type Text))
  (bind (_npcdatahandle_datatable _npcdatahandle_rowname) (break `DataTableRowHandle` (`self.NPCDataHandle`)))
  (bind _returnvalue (`|GetDataTableRow` _npcdatahandle_datatable _npcdatahandle_rowname)
    (:`then`
      (return (`.NPCName_2_A051A075476DA2373044E1899278786C` (break `/Game/SOsQuestAndDialogueSystem/Framework/Blueprints/Stucts/Struct_NPCData` _returnvalue))))))

(fn `GetNPCData`
  (returns (Return :type "/Game/SOsQuestAndDialogueSystem/Framework/Blueprints/Stucts/Struct_NPCData Structure"))
  (locals (NPCData :type "/Game/SOsQuestAndDialogueSystem/Framework/Blueprints/Stucts/Struct_NPCData Structure" :default (struct :`Dialogue` (struct))))
  (bind (_npcdatahandle_datatable _npcdatahandle_rowname) (break `DataTableRowHandle` (`self.NPCDataHandle`)))
  (bind _returnvalue (`|GetDataTableRow` _npcdatahandle_datatable _npcdatahandle_rowname)
    (:`then`
      (bind (_npcname _npc _dialogue) (break `/Game/SOsQuestAndDialogueSystem/Framework/Blueprints/Stucts/Struct_NPCData` _returnvalue))
      (bind _output_get (set `local.NPCData` (make `/Game/SOsQuestAndDialogueSystem/Framework/Blueprints/Stucts/Struct_NPCData` _npcname self _dialogue)))
      (return _output_get))))

(fn `Interact`
  (params (InCharacter :type "Character Object Reference"))
  (bind (_npcname _npc _dialogue) (break `/Game/SOsQuestAndDialogueSystem/Framework/Blueprints/Stucts/Struct_NPCData` (`self.GetNPCData`)))
  (`parent.Interact` InCharacter)
  (bind _asbp_player_character (cast `/Game/SOsQuestAndDialogueSystem/Framework/Blueprints/BP_PlayerCharacter` InCharacter))
  (`/Game/SOsQuestAndDialogueSystem/Blueprints/DialogueSystem/BP_SOsDialogueManager_Component.EnterDialogueWithNPCEx` (`/Game/SOsQuestAndDialogueSystem/Framework/Blueprints/BP_TopDownController.NPCDialogueManager` (`/Game/SOsQuestAndDialogueSystem/Framework/Blueprints/BP_PlayerCharacter.GetPlayerControllerBP` _asbp_player_character)) _npc _dialogue))

(fn `UserConstructionScript`)
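; Quest and dialogue system helper actor that opens the next tutorial area by destroying a door obstacle when it begins play.
; BeginPlay gathers all BP_Obstacle actors and searches by hard-coded Name for the Area 1, 2 and 3 tutorial doors in order, removing only the first found.
; It then sets a short lifespan to remove itself, so each new instance clears at most one door, with no overlap logic involved.
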(event `self.ReceiveBeginPlay`
  (`parent.ReceiveBeginPlay`)
  (bind _outactors (`GameplayStatics.GetAllActorsOfClass` "/Game/SOsQuestAndDialogueSystem/Framework/Blueprints/BP_Obstacle.BP_Obstacle_C"))
  (for _array_element _outactors
    (if (== (`/Game/SOsQuestAndDialogueSystem/Framework/Blueprints/BP_Obstacle.Name` _array_element) "TutorialArea1Door")
      (`self.K2_DestroyActor` _array_element)
      (set `self.Found` true)
      (break)))
  (if (`self.Found`)
    (`self.SetLifeSpan` 1.0)
    (else
      (for _array_element_2 _outactors
        (if (== (`/Game/SOsQuestAndDialogueSystem/Framework/Blueprints/BP_Obstacle.Name` _array_element_2) "TutorialArea2Door")
          (`self.K2_DestroyActor` _array_element_2)
          (set `self.Found` true)
          (break)))
      (if (`self.Found`)
        (`self.SetLifeSpan` 1.0)
        (else
          (for _array_element_3 _outactors
            (if (== (`/Game/SOsQuestAndDialogueSystem/Framework/Blueprints/BP_Obstacle.Name` _array_element_3) "TutorialArea3Door")
              (`self.K2_DestroyActor` _array_element_3)
              (set `self.Found` true)
              (break)))
          (`self.SetLifeSpan` 1.0))))))

(fn `UserConstructionScript`
  (`parent.UserConstructionScript`))
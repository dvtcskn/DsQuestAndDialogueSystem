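; BP_GreenNPC_Trigger is a short-lived helper actor that switches off interaction on the Green NPC.
; On BeginPlay it takes the first BP_EnemyCharacter found in the level and looks up its NPC data table row.
; If that row's name is "GreenNPC", it clears the character's Interactable and EnemyInteractable flags, then sets its own one-second lifespan.
; Only that first enemy is checked, and without a match the trigger stays alive.
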(event `self.ReceiveBeginPlay`
  (`parent.ReceiveBeginPlay`)
  (bind _outactors (`GameplayStatics.GetAllActorsOfClass` "/Game/DsQuestAndDialogueSystem/Framework/Blueprints/BP_EnemyCharacter.BP_EnemyCharacter_C"))
  (bind _output (`|GetArrayItem` _outactors))
  (bind (_npcdatahandle_datatable _npcdatahandle_rowname) (break `DataTableRowHandle` (`/Game/DsQuestAndDialogueSystem/Framework/Blueprints/BP_EnemyCharacter.NPCDataHandle` _output)))
  (bind _returnvalue (`|GetDataTableRow` _npcdatahandle_datatable _npcdatahandle_rowname)
    (:`then`
      (if (`KismetTextLibrary.EqualEqual_TextText` (`.NPCName_2_A051A075476DA2373044E1899278786C` (break `/Game/DsQuestAndDialogueSystem/Framework/Blueprints/Stucts/Struct_NPCData` _returnvalue)) (`KismetTextLibrary.Conv_StringToText` "GreenNPC"))
        (set `/Game/DsQuestAndDialogueSystem/Framework/Blueprints/BP_CharacterBase.Interactable` false _output)
        (set `/Game/DsQuestAndDialogueSystem/Framework/Blueprints/BP_EnemyCharacter.Enemy_Interactable` false _output)
        (`self.SetLifeSpan` 1.0)))))

(fn `UserConstructionScript`
  (`parent.UserConstructionScript`))
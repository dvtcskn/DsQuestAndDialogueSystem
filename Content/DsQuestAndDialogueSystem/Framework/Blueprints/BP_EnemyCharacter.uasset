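; Enemy character for the quest and dialogue system that players can talk to and kill for quest progress.
; Interact and EndInteract start and end conversations through the player controller's NPCDialogueManager, using name and dialogue from a data table row.
; The first damage of at least 1 from a player character progresses the QuestManager with a Fragment, hides the enemy, spawns DeathTrigger at world origin and sets a short lifespan.
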(event `self.ReceiveBeginPlay`
  (set `self.Interactable` (`self.Enemy_Interactable`)))

(event `self.ReceiveAnyDamage`
  (params (Damage :type "Float (single-precision)") (DamageType :type "DamageType Object Reference") (InstigatedBy :type "Controller Object Reference") (DamageCauser :type "Actor Object Reference"))
  (if (>= Damage 1.0)
    (bind _asbp_player_character (cast `/Game/SOsQuestAndDialogueSystem/Framework/Blueprints/BP_PlayerCharacter` DamageCauser))
    (`/Engine/EditorBlueprintResources/StandardMacros.DoOnce` false
      (:`Completed`
        (`/Game/SOsQuestAndDialogueSystem/Blueprints/QuestSystem/BP_SOsQuestManager_Component.ProgressQuest` (`/Game/SOsQuestAndDialogueSystem/Framework/Blueprints/BP_TopDownController.QuestManager` (`/Game/SOsQuestAndDialogueSystem/Framework/Blueprints/BP_PlayerCharacter.GetPlayerControllerBP` _asbp_player_character)) (`self.Fragment`))
        (`self.SetActorHiddenInGame` true)
        (`|SpawnActorFromClass` (`self.DeathTrigger`) (`KismetMathLibrary.MakeTransform` (0.0 0.0 0.0)) "AdjustIfPossibleButAlwaysSpawn" "OverrideRootScale" null null null)
        (`self.SetLifeSpan` 0.5)))))

(fn `EndInteract`
  (params (InCharacter :type "Character Object Reference"))
  (`parent.EndInteract` InCharacter)
  (bind _asbp_player_character (cast `/Game/SOsQuestAndDialogueSystem/Framework/Blueprints/BP_PlayerCharacter` InCharacter))
  (`/Game/SOsQuestAndDialogueSystem/Blueprints/DialogueSystem/BP_SOsDialogueManager_Component.EndCoversation` (`/Game/SOsQuestAndDialogueSystem/Framework/Blueprints/BP_TopDownController.NPCDialogueManager` (`/Game/SOsQuestAndDialogueSystem/Framework/Blueprints/BP_PlayerCharacter.GetPlayerControllerBP` _asbp_player_character))))

(fn `GetName`
  (returns (Return :type Text))
  (bind (_npcdatahandle_datatable _npcdatahandle_rowname) (break `DataTableRowHandle` (`self.NPCDataHandle`)))
  (bind _returnvalue (`|GetDataTableRow` _npcdatahandle_datatable _npcdatahandle_rowname)
    (:`then`
      (return (`.NPCName_2_A051A075476DA2373044E1899278786C` (break `/Game/SOsQuestAndDialogueSystem/Framework/Blueprints/Stucts/Struct_NPCData` _returnvalue))))))

(fn `GetNPCData`
  (returns (Return :type "/Game/SOsQuestAndDialogueSystem/Framework/Blueprints/Stucts/Struct_NPCData Structure"))
  (locals (NPCData :type "/Game/SOsQuestAndDialogueSystem/Framework/Blueprints/Stucts/Struct_NPCData Structure" :default (struct :`Dialogue` (struct))))
  (bind (_npcdatahandle_datatable _npcdatahandle_rowname) (break `DataTableRowHandle` (`self.NPCDataHandle`)))
  (bind _returnvalue (`|GetDataTableRow` _npcdatahandle_datatable _npcdatahandle_rowname)
    (:`then`
      (bind (_npcname _npc _dialogue) (break `/Game/SOsQuestAndDialogueSystem/Framework/Blueprints/Stucts/Struct_NPCData` _returnvalue))
      (bind _output_get (set `local.NPCData` (make `/Game/SOsQuestAndDialogueSystem/Framework/Blueprints/Stucts/Struct_NPCData` _npcname self _dialogue)))
      (return _output_get))))

(fn `Interact`
  (params (InCharacter :type "Character Object Reference"))
  (bind (_npcname _npc _dialogue) (break `/Game/SOsQuestAndDialogueSystem/Framework/Blueprints/Stucts/Struct_NPCData` (`self.GetNPCData`)))
  (`parent.Interact` InCharacter)
  (bind _asbp_player_character (cast `/Game/SOsQuestAndDialogueSystem/Framework/Blueprints/BP_PlayerCharacter` InCharacter))
  (`/Game/SOsQuestAndDialogueSystem/Blueprints/DialogueSystem/BP_SOsDialogueManager_Component.EnterDialogueWithNPCEx` (`/Game/SOsQuestAndDialogueSystem/Framework/Blueprints/BP_TopDownController.NPCDialogueManager` (`/Game/SOsQuestAndDialogueSystem/Framework/Blueprints/BP_PlayerCharacter.GetPlayerControllerBP` _asbp_player_character)) _npc _dialogue))

(fn `UserConstructionScript`)
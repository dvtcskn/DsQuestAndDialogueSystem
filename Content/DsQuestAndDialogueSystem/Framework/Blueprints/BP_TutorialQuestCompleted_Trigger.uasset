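; Trigger actor in the quest and dialogue system that announces a completed tutorial quest when spawned or placed.
; On BeginPlay it casts the player controller to BP_TopDownController and calls ShowCompletedText on its OnScreenWidget.
; After a successful cast it sets a one-second lifespan, so the actor removes itself.
; Despite the Trigger name, its overlap and tick events are disabled, so no overlap is involved.
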(event `self.ReceiveBeginPlay`
  (`parent.ReceiveBeginPlay`)
  (bind _asbp_top_down_controller (cast `/Game/DsQuestAndDialogueSystem/Framework/Blueprints/BP_TopDownController` (`GameplayStatics.GetPlayerController` 0)))
  (`/Game/DsQuestAndDialogueSystem/UI/Widget_OnScreen.ShowCompletedText` (`/Game/DsQuestAndDialogueSystem/Framework/Blueprints/BP_TopDownController.OnScreenWidget` _asbp_top_down_controller))
  (`self.SetLifeSpan` 1.0))

(fn `UserConstructionScript`
  (`parent.UserConstructionScript`))
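; BP_QuestTriggerZone is a box trigger that starts and progresses quests when the player character enters it.
; The first overlap passes a DoOnce, which precedes the player cast, so any overlapping actor uses up the trigger.
; For the player, it calls the controller's QuestManager to start the QuestHandle quest if that row is set.
; It then progresses QuestFragment through the same manager, regardless of whether a quest handle is set.
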(event `self.Box.OnComponentBeginOverlap`
  (params (OverlappedComponent :type "PrimitiveComponent Object Reference") (OtherActor :type "Actor Object Reference") (OtherComp :type "PrimitiveComponent Object Reference") (OtherBodyIndex :type Integer) (bFromSweep :type Boolean) (SweepResult :type "HitResult Structure (by ref)"))
  (bind (_datatable _rowname) (break `DataTableRowHandle` (`self.QuestHandle`)))
  (`/Engine/EditorBlueprintResources/StandardMacros.DoOnce` false
    (:`Completed`
      (`|ExecutionSequence`
        (:`then_0`
          (bind _asbp_player_character (cast `/Game/DsQuestAndDialogueSystem/Framework/Blueprints/BP_PlayerCharacter` OtherActor))
          (`/Engine/EditorBlueprintResources/StandardMacros.IsValid` _datatable
            (:`Is Valid`
              (if (!= _rowname "None")
                (`/Game/DsQuestAndDialogueSystem/Blueprints/QuestSystem/BP_SOsQuestManager_Component.StartQuest` (`/Game/DsQuestAndDialogueSystem/Framework/Blueprints/BP_TopDownController.QuestManager` (`/Game/DsQuestAndDialogueSystem/Framework/Blueprints/BP_PlayerCharacter.GetPlayerControllerBP` _asbp_player_character)) (`self.QuestHandle`))))))
        (:`then_1`
          (bind _asbp_player_character_2 (cast `/Game/DsQuestAndDialogueSystem/Framework/Blueprints/BP_PlayerCharacter` OtherActor))
          (`/Game/DsQuestAndDialogueSystem/Blueprints/QuestSystem/BP_SOsQuestManager_Component.ProgressQuest` (`/Game/DsQuestAndDialogueSystem/Framework/Blueprints/BP_TopDownController.QuestManager` (`/Game/DsQuestAndDialogueSystem/Framework/Blueprints/BP_PlayerCharacter.GetPlayerControllerBP` _asbp_player_character_2)) (`self.QuestFragment`)))))))

(fn `UserConstructionScript`)
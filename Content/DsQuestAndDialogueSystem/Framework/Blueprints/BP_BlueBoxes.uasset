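; BP_BlueBoxes is a pickup item in the quest and dialogue system, a colored box that can be added to a controller's inventory.
; The construction script creates a dynamic material for the cube, and cursor hover events swap its color for highlighting.
; BeginPlay defers to the parent class to create the unique item.
; Pickup runs once, passing that item to the controller, then hiding the actor and expiring it shortly after.
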(event `self.ReceiveBeginPlay`
  ;[1 1 1] Base Class is creating unique item so call parent function
  (`parent.ReceiveBeginPlay`))

(event `self.BeginCursorOver`
  (params (Controller :type "/Game/SOsQuestAndDialogueSystem/Framework/Blueprints/BP_TopDownController Object Reference"))
  (`MaterialInstanceDynamic.SetVectorParameterValue` (`self.DynamicMaterial`) "Color" (`self.HowerColor`)))

(event `self.EndCursorOver`
  (`MaterialInstanceDynamic.SetVectorParameterValue` (`self.DynamicMaterial`) "Color" (`self.Color`)))

(event `self.Pickup`
  (params (Controller :type "/Game/SOsQuestAndDialogueSystem/Framework/Blueprints/BP_TopDownController Object Reference"))
  (`/Engine/EditorBlueprintResources/StandardMacros.DoOnce` false
    (:`Completed`
      (`/Game/SOsQuestAndDialogueSystem/Framework/Blueprints/BP_TopDownController.AddItemToInventory` Controller (`self.GetItem`))
      (`self.SetActorHiddenInGame` true)
      (`self.SetLifeSpan` 0.5))))

(fn `UserConstructionScript`
  (bind _returnvalue (`PrimitiveComponent.CreateDynamicMaterialInstance` (`self.Cube`) 0 "/Game/SOsQuestAndDialogueSystem/Geometry/Meshes/CubeMaterial_Inst.CubeMaterial_Inst" "None"))
  (bind _output_get (set `self.DynamicMaterial` _returnvalue))
  (`MaterialInstanceDynamic.SetVectorParameterValue` _output_get "Color" (`self.Color`)))
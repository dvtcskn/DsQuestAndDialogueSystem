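; BP_CharacterBase is a character base in the quest and dialogue system that highlights its body under the mouse cursor.
; Construction creates a dynamic mannequin material and sets its BodyColor, which capsule cursor-over events swap between hover and normal colors.
; It exposes type and capsule radius getters, plus stub Interact, EndInteract, GetName and GetNPCData functions that do nothing or return empty results.
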(event `self.CapsuleComponent.OnBeginCursorOver`
  (params (TouchedComponent :type "PrimitiveComponent Object Reference"))
  (`MaterialInstanceDynamic.SetVectorParameterValue` (`self.DynamicMaterial`) "BodyColor" (`self.HowerColor`)))

(event `self.CapsuleComponent.OnEndCursorOver`
  (params (TouchedComponent :type "PrimitiveComponent Object Reference"))
  (`MaterialInstanceDynamic.SetVectorParameterValue` (`self.DynamicMaterial`) "BodyColor" (`self.Color`)))

(fn `EndInteract`
  (params (InCharacter :type "Character Object Reference")))

(fn `GetName`
  (returns (Return :type Text))
  (return ""))

(fn `GetNPCData`
  (returns (Return :type "/Game/DsQuestAndDialogueSystem/Framework/Blueprints/Stucts/Struct_NPCData Structure"))
  (return))

(fn `GetRadius`
  (params (Scaled :type Boolean))
  (returns (Return :type "Float (double-precision)"))
  (bind _capsulecomponent (`self.CapsuleComponent`))
  (if Scaled
    (return (`CapsuleComponent.GetScaledCapsuleRadius` _capsulecomponent))
    (else
      (return (`CapsuleComponent.GetUnscaledCapsuleRadius` _capsulecomponent)))))

(fn `GetType`
  (returns (Type :type "/Game/DsQuestAndDialogueSystem/Framework/Blueprints/Enums/Enum_CharacterType Enum"))
  (return (`self.Type`)))

(fn `Interact`
  (params (InCharacter :type "Character Object Reference")))

(fn `UserConstructionScript`
  (bind _returnvalue (`PrimitiveComponent.CreateDynamicMaterialInstance` (`self.Mesh`) 0 "/Game/DsQuestAndDialogueSystem/Mannequin/Character/Materials/M_UE4Man_Body_Inst.M_UE4Man_Body_Inst" "None"))
  (set `self.DynamicMaterial` _returnvalue)
  (`MaterialInstanceDynamic.SetVectorParameterValue` (`self.DynamicMaterial`) "BodyColor" (`self.Color`)))
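; Scripted trigger actor that, once spawned, sends the NPC named "BlackNPC" to the player and opens a conversation.
; BeginPlay finds that NPC by its data table name, then orders its AI controller to pathfind to the player character.
; On move completion, regardless of result, a DoOnce ends any current conversation, starts the NPC's data table dialogue and sets a short lifespan on the trigger.
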(event `self.ReceiveBeginPlay`
  (`parent.ReceiveBeginPlay`)
  (bind _outactors (`GameplayStatics.GetAllActorsOfClass` "/Game/DsQuestAndDialogueSystem/Framework/Blueprints/BP_NPC_Character.BP_NPC_Character_C"))
  (for _array_element _outactors
    (bind (_npcdatahandle_datatable _npcdatahandle_rowname) (break `DataTableRowHandle` (`/Game/DsQuestAndDialogueSystem/Framework/Blueprints/BP_NPC_Character.NPCDataHandle` _array_element)))
    (bind _returnvalue (`|GetDataTableRow` _npcdatahandle_datatable _npcdatahandle_rowname)
      (:`then`
        (if (`KismetTextLibrary.EqualEqual_TextText` (`.NPCName_2_A051A075476DA2373044E1899278786C` (break `/Game/DsQuestAndDialogueSystem/Framework/Blueprints/Stucts/Struct_NPCData` _returnvalue)) (`KismetTextLibrary.Conv_StringToText` "BlackNPC"))
          (set `self.BlackNPC` _array_element)))))
  (bind _outactors_2 (`GameplayStatics.GetAllActorsOfClass` "/Game/DsQuestAndDialogueSystem/Framework/Blueprints/BP_PlayerCharacter.BP_PlayerCharacter_C"))
  (set `self.PlayerCharacter` (`|GetArrayItem` _outactors_2))
  (bind _asbp_player_aicontroller (cast `/Game/DsQuestAndDialogueSystem/Framework/Blueprints/BP_PlayerAIController` (`AIBlueprintHelperLibrary.GetAIController` (`self.BlackNPC`))))
  (add `/Game/DsQuestAndDialogueSystem/Framework/Blueprints/BP_PlayerAIController.AIMoveToCompletedSignature` _asbp_player_aicontroller (delegate `AIMoveToCompletedSignature_Event_0`))
  (`/Game/DsQuestAndDialogueSystem/Framework/Blueprints/BP_PlayerAIController.AIMoveToActor` _asbp_player_aicontroller (`self.PlayerCharacter`) 42.0 false true false false))

(event `AIMoveToCompletedSignature_Event_0`
  (params (InActor :type "Actor Object Reference") (PathFollowingResult :type "EPathFollowingResult Enum" :default "Success"))
  (bind (_npcdatahandle_datatable _npcdatahandle_rowname) (break `DataTableRowHandle` (`/Game/DsQuestAndDialogueSystem/Framework/Blueprints/BP_NPC_Character.NPCDataHandle` (`self.BlackNPC`))))
  (bind _npcdialoguemanager (`/Game/DsQuestAndDialogueSystem/Framework/Blueprints/BP_TopDownController.NPCDialogueManager` (`/Game/DsQuestAndDialogueSystem/Framework/Blueprints/BP_PlayerCharacter.GetPlayerControllerBP` (`self.PlayerCharacter`))))
  (`/Engine/EditorBlueprintResources/StandardMacros.DoOnce` false
    (:`Completed`
      (`/Game/DsQuestAndDialogueSystem/Blueprints/DialogueSystem/BP_SOsDialogueManager_Component.EndCoversation` _npcdialoguemanager)
      (bind _returnvalue (`|GetDataTableRow` _npcdatahandle_datatable _npcdatahandle_rowname)
        (:`then`
          (`/Game/DsQuestAndDialogueSystem/Blueprints/DialogueSystem/BP_SOsDialogueManager_Component.EnterDialogueWithNPCEx` _npcdialoguemanager (`self.BlackNPC`) (`.Dialogue_8_AEEA24E14B7D80E0322C93928EAF0F3D` (break `/Game/DsQuestAndDialogueSystem/Framework/Blueprints/Stucts/Struct_NPCData` _returnvalue)))
          (`self.SetLifeSpan` 5.0))))))

(fn `UserConstructionScript`
  (`parent.UserConstructionScript`))
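; Base pickup actor for the quest and dialogue system, representing an item that child Blueprints make collectible.
; On BeginPlay it looks up its handle in DT_ItemList and wraps the row in a BP_DSsItemInfo object.
; Pickup and cursor-over events are empty override hooks, and a sphere component supplies the radius.
; Two helpers query a quest manager for the item's bound quests, one also checking that the matching parameter is incomplete.
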(event `self.ReceiveBeginPlay`
  (bind (_itemhandle_datatable _itemhandle_rowname) (break `DataTableRowHandle` (`self.ItemHandle`)))
  ;[1 1 1] All items needs to be unique
  (bind _returnvalue (`|GetDataTableRow` "/Game/DsQuestAndDialogueSystem/Framework/Blueprints/Data/DT_ItemList.DT_ItemList" _itemhandle_rowname)
    (:`then`
      (bind _returnvalue_2 (`|GenericCreateObject` self "/Game/DsQuestAndDialogueSystem/Blueprints/FrameworkOnly/BP_DSsItemInfo.BP_DSsItemInfo_C" _returnvalue))
      (set `self.Item` _returnvalue_2))))

(event `Pickup`
  (params (Controller :type "/Game/DsQuestAndDialogueSystem/Framework/Blueprints/BP_TopDownController Object Reference"))
  ;[1 1 1] Override this events
)

(event `BeginCursorOver`
  (params (Controller :type "/Game/DsQuestAndDialogueSystem/Framework/Blueprints/BP_TopDownController Object Reference"))
  ;[1 1 1] Override this events
)

(event `EndCursorOver`
  ;[1 1 1] Override this events
)

(fn `CheckReqQuestAndParameterIsActive`
  (params (QuestManager :type "/Game/DsQuestAndDialogueSystem/Blueprints/QuestSystem/BP_DSsQuestManager_Component Object Reference"))
  (returns (Return :type Boolean))
  (bind (_type _id _value _boundtoquests) (break `/Game/DsQuestAndDialogueSystem/Blueprints/Structs/Quest/Struct_DSsQuestFragment` (`.QuestFragment_22_94AE95B24814A21B53FA7A899A100156` (break `/Game/DsQuestAndDialogueSystem/Blueprints/Structs/Framework/Struct_DSsItemInfoBase` (`/Game/DsQuestAndDialogueSystem/Blueprints/FrameworkOnly/BP_DSsItemInfo.ItemInfo` (`self.Item`))))))
  (for _array_element _boundtoquests
    (bind _returnvalue (`|GetDataTableRow` (break `DataTableRowHandle` _array_element) (`.RowName` (break `DataTableRowHandle` _array_element)))
      (:`then`
        (bind _quest (`/Game/DsQuestAndDialogueSystem/Blueprints/QuestSystem/BP_DSsQuestManager_Component.GetQuestByID` QuestManager "NewEnumerator0" (`.QuestID_4_4DA48B5A4D4871FBE8DA14A70DAE74DD` (break `/Game/DsQuestAndDialogueSystem/Blueprints/Structs/Quest/Struct_DSsQuestFramework` _returnvalue))))
        (`/Engine/EditorBlueprintResources/StandardMacros.IsValid` _quest
          (:`Is Valid`
            (return (not (`/Game/DsQuestAndDialogueSystem/Blueprints/QuestSystem/BP_DSsQuestParameterBase.GetIsCompleted` (`/Game/DsQuestAndDialogueSystem/Blueprints/QuestSystem/BP_DSsQuestBase.GetParameterByFragmentID` _quest _id)))))))))
  (return false))

(fn `CheckReqQuestIsActive`
  (params (QuestManager :type "/Game/DsQuestAndDialogueSystem/Blueprints/QuestSystem/BP_DSsQuestManager_Component Object Reference"))
  (returns (Return :type Boolean))
  (for _array_element (`.BoundToQuests_19_7512147C43A2FC7F3B0E5EAC5042E095` (break `/Game/DsQuestAndDialogueSystem/Blueprints/Structs/Quest/Struct_DSsQuestFragment` (`.QuestFragment_22_94AE95B24814A21B53FA7A899A100156` (break `/Game/DsQuestAndDialogueSystem/Blueprints/Structs/Framework/Struct_DSsItemInfoBase` (`/Game/DsQuestAndDialogueSystem/Blueprints/FrameworkOnly/BP_DSsItemInfo.ItemInfo` (`self.Item`))))))
    (bind _returnvalue (`|GetDataTableRow` (break `DataTableRowHandle` _array_element) (`.RowName` (break `DataTableRowHandle` _array_element)))
      (:`then`
        (bind _quest (`/Game/DsQuestAndDialogueSystem/Blueprints/QuestSystem/BP_DSsQuestManager_Component.GetQuestByID` QuestManager "NewEnumerator0" (`.QuestID_4_4DA48B5A4D4871FBE8DA14A70DAE74DD` (break `/Game/DsQuestAndDialogueSystem/Blueprints/Structs/Quest/Struct_DSsQuestFramework` _returnvalue))))
        (`/Engine/EditorBlueprintResources/StandardMacros.IsValid` _quest
          (:`Is Valid`
            (return true))))))
  (return false))

(fn `GetItem`
  (returns (Item :type "/Game/DsQuestAndDialogueSystem/Blueprints/FrameworkOnly/BP_DSsItemInfo Object Reference"))
  (return (`self.Item`)))

(fn `GetRadius`
  (params (Scaled :type Boolean))
  (returns (ReturnValue :type "Float (double-precision)"))
  (bind _sphere (`self.Sphere`))
  (if Scaled
    (return (`SphereComponent.GetScaledSphereRadius` _sphere))
    (else
      (return (`SphereComponent.GetUnscaledSphereRadius` _sphere)))))

(fn `UserConstructionScript`)
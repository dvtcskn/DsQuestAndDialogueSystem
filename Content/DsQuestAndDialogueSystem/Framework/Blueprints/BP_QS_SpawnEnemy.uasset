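; BP_QS_SpawnEnemy is a short-lived spawner that places enemies for the orange NPC kill quest.
; On BeginPlay it finds all BP_SpawnZone actors and spawns a BP_EnemyCharacter at each of the first two.
; Each enemy receives the spawner's colors and a quest fragment bound to the kill quest's DT_Quest row.
; The spawner then sets a brief lifespan so it removes itself.
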(event `self.ReceiveBeginPlay`
  (bind _struct_sosquestfragment (make `/Game/DsQuestAndDialogueSystem/Blueprints/Structs/Quest/Struct_SOsQuestFragment` "NewEnumerator4" "SQ_ON-1" 1.0 (`|MakeArray` (make `DataTableRowHandle` "/Game/DsQuestAndDialogueSystem/Framework/Blueprints/Data/DT_Quest.DT_Quest" "SQ_OrangeNPC_KillQuest"))))
  (`parent.ReceiveBeginPlay`)
  (bind _outactors (`GameplayStatics.GetAllActorsOfClass` "/Game/DsQuestAndDialogueSystem/Framework/Blueprints/BP_SpawnZone.BP_SpawnZone_C"))
  (`|SpawnActorFromClass` "/Game/DsQuestAndDialogueSystem/Framework/Blueprints/BP_EnemyCharacter.BP_EnemyCharacter_C" (`KismetMathLibrary.MakeTransform` (`self.K2_GetActorLocation` (`|GetArrayItem` _outactors))) "AlwaysSpawn" "MultiplyWithRoot" null _struct_sosquestfragment false null (struct) null (`self.Color`) (`self.HowerColor`) null)
  (`|SpawnActorFromClass` "/Game/DsQuestAndDialogueSystem/Framework/Blueprints/BP_EnemyCharacter.BP_EnemyCharacter_C" (`KismetMathLibrary.MakeTransform` (`self.K2_GetActorLocation` (`|GetArrayItem` _outactors 1))) "AlwaysSpawn" "MultiplyWithRoot" null _struct_sosquestfragment false null (struct) null (`self.Color`) (`self.HowerColor`) null)
  (`self.SetLifeSpan` 2.0))

(fn `UserConstructionScript`
  (`parent.UserConstructionScript`))
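; Player-controlled proxy for top-down click-to-move play that spawns BP_PlayerCharacter, attaches itself to it and forwards possession and movement commands.
; The MouseX axis event traces under the cursor to update pickup hover and, while left mouse is held, targets characters, pickups or ground points.
; An AI-controller range check decides between walking to a target and acting on it: pickup, NPC interaction or enemy attack.
; A blocking flag suppresses movement.
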(event `InputAxisKey|MouseX`
  (params (AxisValue :type "Float (single-precision)"))
  (bind _pickupactor (`self.PickupActor`))
  (bind _asbp_pick_up_base (cast `/Game/SOsQuestAndDialogueSystem/Framework/Blueprints/BP_PickUpBase` (`.HitActor` (`GameplayStatics.BreakHitResult` (`PlayerController.GetHitResultUnderCursorByChannel` (`self.Get Player ControllerBP`) "TraceTypeQuery1" true))))
    (:`then`
      (if (and (!= _asbp_pick_up_base _pickupactor) (`KismetSystemLibrary.IsValid` _pickupactor))
        (`/Game/SOsQuestAndDialogueSystem/Framework/Blueprints/BP_PickUpBase.EndCursorOver` (`self.PickupActor`)))
      (bind _output_get (set `self.PickupActor` _asbp_pick_up_base))
      (`/Game/SOsQuestAndDialogueSystem/Framework/Blueprints/BP_PickUpBase.BeginCursorOver` _output_get (`self.Get Player ControllerBP`)))
    (:`CastFailed`
      (`/Engine/EditorBlueprintResources/StandardMacros.IsValid` (`self.PickupActor`)
        (:`Is Valid`
          (`/Game/SOsQuestAndDialogueSystem/Framework/Blueprints/BP_PickUpBase.EndCursorOver` (`self.PickupActor`)))
        (:`Is Not Valid`
          _))
      (set `self.PickupActor` null)))
  (if (`self.LeftMouseButton_Clicked`)
    (`/Engine/EditorBlueprintResources/StandardMacros.IsValid` (`self.PlayerCharacter`)
      (:`Is Valid`
        (`self.LeftMouseButtonDown`)))))

(event `Key|LeftMouseButton`
  (params (Key :type "Key Structure"))
  (:`Pressed`
    (set `self.LeftMouseButton_Clicked` true))
  (:`Released`
    (set `self.LeftMouseButton_Clicked` false)))

(event `Key|RightMouseButton`
  (params (Key :type "Key Structure")))

(event `self.ReceiveBeginPlay`
  (`/Game/SOsQuestAndDialogueSystem/Framework/Blueprints/BP_TopDownController.RegisterPlayerCharacterController` (`self.Get Player ControllerBP`) self)
  (bind _returnvalue (`|SpawnActorFromClass` "/Game/SOsQuestAndDialogueSystem/Framework/Blueprints/BP_PlayerCharacter.BP_PlayerCharacter_C" (`KismetMathLibrary.MakeTransform` (`self.K2_GetActorLocation`)) "Undefined" "OverrideRootScale" self null))
  (`self.SetOwner` _returnvalue self)
  (`self.RegisterPlayerCharacter` _returnvalue))

(event `self.ReceiveTick`
  (params (DeltaSeconds :type "Float (single-precision)")))

(fn `BlockMovementInput`
  (params (value :type Boolean))
  (bind _playercharacter (`self.PlayerCharacter`))
  (set `self.bBlockedMovement` value)
  (`/Engine/EditorBlueprintResources/StandardMacros.IsValid` _playercharacter
    (:`Is Valid`
      (`/Game/SOsQuestAndDialogueSystem/Framework/Blueprints/BP_PlayerCharacter.StopMovement` _playercharacter))))

(fn `Get Player ControllerBP`
  (returns (Controller :type "/Game/SOsQuestAndDialogueSystem/Framework/Blueprints/BP_TopDownController Object Reference"))
  (return (cast `/Game/SOsQuestAndDialogueSystem/Framework/Blueprints/BP_TopDownController` (`self.GetController`) :!pure true)))

(fn `InteractTarget`
  (params (Character :type "/Game/SOsQuestAndDialogueSystem/Framework/Blueprints/BP_CharacterBase Object Reference"))
  ;[1 1 1] Interact with target or attack
  (switch `/Game/SOsQuestAndDialogueSystem/Framework/Blueprints/Enums/Enum_CharacterType` (`/Game/SOsQuestAndDialogueSystem/Framework/Blueprints/BP_CharacterBase.GetType` Character)
    (:`NewEnumerator2`
      (if (`/Game/SOsQuestAndDialogueSystem/Framework/Blueprints/BP_CharacterBase.Interactable` Character)
        (`/Game/SOsQuestAndDialogueSystem/Framework/Blueprints/BP_PlayerCharacter.EndInteractNPC` (`self.PlayerCharacter`))
        (`/Game/SOsQuestAndDialogueSystem/Framework/Blueprints/BP_PlayerCharacter.InteractNPC` (`self.PlayerCharacter`) Character)
        (else
          (`/Game/SOsQuestAndDialogueSystem/Framework/Blueprints/BP_PlayerCharacter.AttacktotheEnemy` (`self.PlayerCharacter`) Character))))
    (:`NewEnumerator3`
      (`/Game/SOsQuestAndDialogueSystem/Framework/Blueprints/BP_PlayerCharacter.EndInteractNPC` (`self.PlayerCharacter`))
      (`/Game/SOsQuestAndDialogueSystem/Framework/Blueprints/BP_PlayerCharacter.InteractNPC` (`self.PlayerCharacter`) Character))))

(fn `LeftMouseButtonDown`
  (bind _hitresult (`PlayerController.GetHitResultUnderCursorByChannel` (`self.Get Player ControllerBP`) "TraceTypeQuery1" true))
  (if (not (`self.bBlockedMovement`))
    (bind _asbp_character_base (cast `/Game/SOsQuestAndDialogueSystem/Framework/Blueprints/BP_CharacterBase` (`.HitActor` (`GameplayStatics.BreakHitResult` _hitresult)))
      (:`then`
        (`self.MoveToActor` _asbp_character_base))
      (:`CastFailed`
        (bind _asbp_pick_up_base (cast `/Game/SOsQuestAndDialogueSystem/Framework/Blueprints/BP_PickUpBase` (`.HitActor` (`GameplayStatics.BreakHitResult` _hitresult)))
          (:`then`
            (`self.MoveToActor` _asbp_pick_up_base))
          (:`CastFailed`
            (`self.MoveTo` (`.ImpactPoint` (`GameplayStatics.BreakHitResult` _hitresult)))))))))

(fn `MoveTo`
  (params (Loc :type "Vector Structure"))
  (bind _playercharacter (`self.PlayerCharacter`))
  (if (not (`self.bBlockedMovement`))
    (`/Engine/EditorBlueprintResources/StandardMacros.IsValid` _playercharacter
      (:`Is Valid`
        (`/Game/SOsQuestAndDialogueSystem/Framework/Blueprints/BP_PlayerCharacter.MoveToLocation` _playercharacter Loc)))))

(fn `MoveToActor`
  (params (InActor :type "Actor Object Reference"))
  (bind _playercharacter (`self.PlayerCharacter`))
  ;[1 1 1] If the character is where the target is, interact with the target or pick up target item. If the character is not on the target, go to the target.
  (`/Engine/EditorBlueprintResources/StandardMacros.IsValid` _playercharacter
    (:`Is Valid`
      (bind _asbp_character_base (cast `/Game/SOsQuestAndDialogueSystem/Framework/Blueprints/BP_CharacterBase` InActor)
        (:`then`
          (if (`/Game/SOsQuestAndDialogueSystem/Framework/Blueprints/BP_PlayerAIController.IsTargetAtTheGoal` (`/Game/SOsQuestAndDialogueSystem/Framework/Blueprints/BP_PlayerCharacter.GetAIControllerBP` (`self.PlayerCharacter`)) (`self.K2_GetActorLocation` _asbp_character_base) (`/Game/SOsQuestAndDialogueSystem/Framework/Blueprints/BP_CharacterBase.GetRadius` _asbp_character_base true) 10.0)
            (`self.InteractTarget` _asbp_character_base)
            (elif (not (`self.bBlockedMovement`))
              (`/Game/SOsQuestAndDialogueSystem/Framework/Blueprints/BP_PlayerCharacter.MoveToActor` _playercharacter InActor (`/Game/SOsQuestAndDialogueSystem/Framework/Blueprints/BP_CharacterBase.GetRadius` _asbp_character_base true)))))
        (:`CastFailed`
          (bind _asbp_pick_up_base (cast `/Game/SOsQuestAndDialogueSystem/Framework/Blueprints/BP_PickUpBase` InActor))
          (if (`/Game/SOsQuestAndDialogueSystem/Framework/Blueprints/BP_PlayerAIController.IsTargetAtTheGoal` (`/Game/SOsQuestAndDialogueSystem/Framework/Blueprints/BP_PlayerCharacter.GetAIControllerBP` (`self.PlayerCharacter`)) (`self.K2_GetActorLocation` _asbp_pick_up_base) (`/Game/SOsQuestAndDialogueSystem/Framework/Blueprints/BP_PickUpBase.GetRadius` _asbp_pick_up_base true) 10.0)
            (`/Game/SOsQuestAndDialogueSystem/Framework/Blueprints/BP_PickUpBase.Pickup` _asbp_pick_up_base (`self.Get Player ControllerBP`))
            (elif (not (`self.bBlockedMovement`))
              (`/Game/SOsQuestAndDialogueSystem/Framework/Blueprints/BP_PlayerCharacter.MoveToActor` _playercharacter InActor (`SphereComponent.GetUnscaledSphereRadius` (`/Game/SOsQuestAndDialogueSystem/Framework/Blueprints/BP_PickUpBase.Sphere` _asbp_pick_up_base))))))))))

(fn `OnPossessed`
  (params (NewController :type "PlayerController Object Reference"))
  (`/Engine/EditorBlueprintResources/StandardMacros.IsValid` (`self.PlayerCharacter`)
    (:`Is Valid`
      (`/Game/SOsQuestAndDialogueSystem/Framework/Blueprints/BP_PlayerCharacter.OnPossessed` (`self.PlayerCharacter`) NewController))))

(fn `OnUnPossessed`
  (`/Engine/EditorBlueprintResources/StandardMacros.IsValid` (`self.PlayerCharacter`)
    (:`Is Valid`
      (`/Game/SOsQuestAndDialogueSystem/Framework/Blueprints/BP_PlayerCharacter.OnUnPossessed` (`self.PlayerCharacter`)))))

(fn `RegisterPlayerCharacter`
  (params (PlayerCharacter :type "/Game/SOsQuestAndDialogueSystem/Framework/Blueprints/BP_PlayerCharacter Object Reference"))
  ;[1 1 1] Player controller communication
  (set `self.PlayerCharacter` PlayerCharacter)
  (`self.OnPossessed` (`self.Get Player ControllerBP`))
  (`self.K2_AttachToActor` (`self.PlayerCharacter`) "None" "SnapToTarget" "KeepRelative" "KeepRelative" false))

(fn `UserConstructionScript`)
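; AI controller that moves the controlled player or base character to a location or actor and signals arrival.
; Its move events store the goal and radius, then call MoveToLocation or MoveToActor.
; Tick polls while movement is idle and broadcasts completion, only ever as Success, when horizontal distance is within range.
; Actor goals add capsule radius and tolerance to that range, while location goals use only the acceptance radius.
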(event `self.ReceiveBeginPlay`)

(event `self.ReceiveTick`
  (params (DeltaSeconds :type "Float (single-precision)"))
  ;[1 1 1] Check if move is completed
  (if (`|EnumEquality` (`self.GetMoveStatus`) "Idle")
    (`/Engine/EditorBlueprintResources/StandardMacros.IsValid` (`self.TempTargetActor`)
      (:`Is Valid`
        (if (<= (`self.DistanceBetweenTargets` (`self.K2_GetActorLocation` (`self.GetPlayerCharacter`)) (`self.K2_GetActorLocation` (`self.TempTargetActor`))) (+ (`CapsuleComponent.GetUnscaledCapsuleRadius` (`Character.CapsuleComponent` (`self.GetPlayerCharacter`))) (`self.Radius`) (`self.Tolerance`)))
          (`self.AIMoveToCompletedSignature` (`self.TempTargetActor`) "Success")))
      (:`Is Not Valid`
        (if (and (<= (`self.DistanceBetweenTargets` (`self.K2_GetActorLocation` (`self.GetPlayerCharacter`)) (`self.Destination`)) (`self.Radius`)) (`KismetMathLibrary.NotEqualExactly_VectorVector` (`self.Destination`)))
          (`self.AIMoveToCompletedSignature` (`self.EmptyTargetActor`) "Success"))))))

(event `AIMoveTo`
  (params (GoalLocation :type "Vector Structure") (AcceptanceRadius :type "Float (double-precision)") (bStopOnOverlap :type Boolean) (bUsePathfinding :type Boolean) (bProjectDestinationToNavigation :type Boolean) (bCanStrafe :type Boolean) (bAllowPartialPath :type Boolean))
  ;[1 1 1] Move
  (set `self.Destination` GoalLocation)
  (set `self.Radius` AcceptanceRadius)
  (set `self.TempTargetActor` (`self.EmptyTargetActor`))
  (`self.MoveToLocation` GoalLocation AcceptanceRadius bStopOnOverlap bUsePathfinding bProjectDestinationToNavigation bCanStrafe null bAllowPartialPath))

(event `AIMoveToActor`
  (params (GoalActor :type "Actor Object Reference") (AcceptanceRadius :type "Float (double-precision)") (bStopOnOverlap :type Boolean) (bUsePathfinding :type Boolean) (bCanStrafe :type Boolean) (bAllowPartialPath :type Boolean))
  ;[1 1 1] Move
  (`/Engine/EditorBlueprintResources/StandardMacros.IsValid` GoalActor
    (:`Is Valid`
      (set `self.TempTargetActor` GoalActor)
      (set `self.Radius` AcceptanceRadius)
      (set `self.Destination` (0.0 0.0 0.0))
      (`self.MoveToActor` GoalActor AcceptanceRadius bStopOnOverlap bUsePathfinding bCanStrafe null bAllowPartialPath))))

(fn `DistanceBetweenTargets`
  (params (V1 :type "Vector Structure") (V2 :type "Vector Structure"))
  (returns (Return :type "Float (double-precision)"))
  (return (`KismetMathLibrary.Sqrt` (+ (`KismetMathLibrary.Square` (- (.x V2) (.x V1))) (`KismetMathLibrary.Square` (- (.y V2) (.y V1)))))))

(fn `GetPlayerCharacter`
  (returns (Character :type "Character Object Reference"))
  (bind _asbp_player_character (cast `/Game/SOsQuestAndDialogueSystem/Framework/Blueprints/BP_PlayerCharacter` (`self.K2_GetPawn`))
    (:`then`
      (return _asbp_player_character))
    (:`CastFailed`
      (bind _asbp_character_base (cast `/Game/SOsQuestAndDialogueSystem/Framework/Blueprints/BP_CharacterBase` (`self.K2_GetPawn`)))
      (return _asbp_character_base))))

(fn `IsTargetAtTheGoal`
  (params (InDestination :type "Vector Structure") (InRadius :type "Float (double-precision)") (InTolerance :type "Float (double-precision)"))
  (returns (return :type Boolean))
  (if (<= (`self.DistanceBetweenTargets` (`self.K2_GetActorLocation` (`self.GetPlayerCharacter`)) InDestination) (+ (`CapsuleComponent.GetUnscaledCapsuleRadius` (`Character.CapsuleComponent` (`self.GetPlayerCharacter`))) InRadius InTolerance))
    (return true)
    (else
      (return false))))

(fn `UserConstructionScript`)
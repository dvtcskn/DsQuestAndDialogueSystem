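; Base object for a single quest objective parameter, tracking progress toward a required amount along with completion, visibility and status.
; Fragments and items with matching IDs raise or lower the clamped value, and consuming an item marks its fragment consumed or adjusts its leftover value.
; Forced completion, visibility and status changes broadcast ParameterUpdated.
; The owning quest section, found through the outer object, handles advancing to the next parameter.
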(fn `AddUniqueParameterID`
  (params (UniqueParameterID :type String))
  (`KismetArrayLibrary.Array_Add` (`.CorrespondingUniqueParameterIDs_14_03DD5036465675D42860EA8589D17ED8` (break `/Game/DsQuestAndDialogueSystem/Blueprints/Structs/Quest/Struct_DSsQuestParameterBaseFramework` (`self.Parameter`))) UniqueParameterID))

(fn `CallNextParameter`
  (`/Game/DsQuestAndDialogueSystem/Blueprints/QuestSystem/BP_DSsQuestSectionBase.CallNextParameter` (`self.GetSection`) self))

(fn `CheckID`
  (params (ID :type "String (by ref)"))
  (returns (return :type Boolean))
  (bind (_parameter_description _parameter_correspondinguniqueparameterids) (break `/Game/DsQuestAndDialogueSystem/Blueprints/Structs/Quest/Struct_DSsQuestParameterBaseFramework` (`self.Parameter`)))
  (return (`KismetArrayLibrary.Array_Contains` _parameter_correspondinguniqueparameterids ID)))

(fn `ConsumeItem`
  (params (Item :type "/Game/DsQuestAndDialogueSystem/Blueprints/FrameworkOnly/BP_DSsItemInfo Object Reference"))
  (returns (Output :type Boolean))
  (bind ((`RequiredAmount_41_289429B5464A19ED43DB2593B832DFC4` _requiredamount)) (break `/Game/DsQuestAndDialogueSystem/Blueprints/Structs/Quest/Struct_DSsQuestParameterBaseFramework` (`self.Parameter`)))
  (bind ((`QuestFragment_22_94AE95B24814A21B53FA7A899A100156` _questfragment)) (break `/Game/DsQuestAndDialogueSystem/Blueprints/Structs/Framework/Struct_DSsItemInfoBase` (`/Game/DsQuestAndDialogueSystem/Blueprints/FrameworkOnly/BP_DSsItemInfo.ItemInfo` Item)))
  (bind (_type _id _value _boundtoquests _consumed) (break `/Game/DsQuestAndDialogueSystem/Blueprints/Structs/Quest/Struct_DSsQuestFragment` _questfragment))
  (bind _returnvalue (- (`self.CurrentValue`) _value))
  ;[1 1 1] Determine whether recorded quest item will be removed or not. If quest item value less than current parameter value it will be consumed and removed.
  (if (`self.CheckID` _id)
    (if (!= (`self.CurrentValue`) 0.0)
      (set `self.IsCompleted` false)
      (if (>= (`self.CurrentValue`) _value)
        (set `self.CurrentValue` _returnvalue)
        (`|VariableSetRef` _questfragment (make `/Game/DsQuestAndDialogueSystem/Blueprints/Structs/Quest/Struct_DSsQuestFragment` _type _id _value _boundtoquests true))
        (else
          (set `self.CurrentValue` _returnvalue)
          (`|VariableSetRef` _questfragment (make `/Game/DsQuestAndDialogueSystem/Blueprints/Structs/Quest/Struct_DSsQuestFragment` _type _id (+ _value (`self.CurrentValue`)) _boundtoquests _consumed))))
      (if (< (`self.CurrentValue`) 0.0)
        (set `self.CurrentValue` 0.0))
      (if (>= (`self.CurrentValue`) _requiredamount)
        (set `self.CurrentValue` _requiredamount)
        (set `self.IsCompleted` true)
        (return true)
        (else
          (return true))))
    (else
      (return false))))

(fn `Decrement`
  (params (Fragment :type "/Game/DsQuestAndDialogueSystem/Blueprints/Structs/Quest/Struct_DSsQuestFragment Structure (by ref)"))
  (returns (Return :type Boolean))
  (bind (_type _id _value) (break `/Game/DsQuestAndDialogueSystem/Blueprints/Structs/Quest/Struct_DSsQuestFragment` Fragment))
  (bind _currentvalue (`self.CurrentValue`))
  (bind _returnvalue (- _currentvalue _value))
  (if (`self.CheckID` _id)
    (set `self.IsCompleted` false)
    (if (> _value _currentvalue)
      (set `self.CurrentValue` _returnvalue)
      (else
        (set `self.CurrentValue` _returnvalue)))
    (if (< (`self.CurrentValue`) 0.0)
      (set `self.CurrentValue` 0.0))
    (return true)
    (else
      (return false))))

(fn `DecrementByItem`
  (params (Item :type "/Game/DsQuestAndDialogueSystem/Blueprints/FrameworkOnly/BP_DSsItemInfo Object Reference (by ref)"))
  (returns (Return :type Boolean))
  (bind _currentvalue (`self.CurrentValue`))
  (bind (_type _id _value) (break `/Game/DsQuestAndDialogueSystem/Blueprints/Structs/Quest/Struct_DSsQuestFragment` (`.QuestFragment_22_94AE95B24814A21B53FA7A899A100156` (break `/Game/DsQuestAndDialogueSystem/Blueprints/Structs/Framework/Struct_DSsItemInfoBase` (`/Game/DsQuestAndDialogueSystem/Blueprints/FrameworkOnly/BP_DSsItemInfo.ItemInfo` Item)))))
  (bind _returnvalue (- _currentvalue _value))
  (if (`self.CheckID` _id)
    (set `self.IsCompleted` false)
    (if (> _value _currentvalue)
      (set `self.CurrentValue` _returnvalue)
      (else
        (set `self.CurrentValue` _returnvalue)))
    (if (< (`self.CurrentValue`) 0.0)
      (set `self.CurrentValue` 0.0))
    (return true)
    (else
      (return false))))

(fn `ForceCompleteParameter`
  (set `self.IsCompleted` true)
  (set `self.CurrentValue` (`.RequiredAmount_41_289429B5464A19ED43DB2593B832DFC4` (break `/Game/DsQuestAndDialogueSystem/Blueprints/Structs/Quest/Struct_DSsQuestParameterBaseFramework` (`self.Parameter`))))
  (`self.ParameterUpdated` self "NewEnumerator2"))

(fn `GetCurrentValue`
  (returns (Float :type "Float (double-precision)"))
  (return (`self.CurrentValue`)))

(fn `GetDescription`
  (returns (Description :type String))
  (bind _parameter_description (break `/Game/DsQuestAndDialogueSystem/Blueprints/Structs/Quest/Struct_DSsQuestParameterBaseFramework` (`self.Parameter`)))
  (return _parameter_description))

(fn `GetIsCompleted`
  (returns (return :type Boolean))
  (return (`self.IsCompleted`)))

(fn `GetIsFailed`
  (returns (return :type Boolean))
  (return (`self.IsFailed`)))

(fn `GetParameterIDs`
  (returns (return :type "Array of String"))
  (return (`.CorrespondingUniqueParameterIDs_14_03DD5036465675D42860EA8589D17ED8` (break `/Game/DsQuestAndDialogueSystem/Blueprints/Structs/Quest/Struct_DSsQuestParameterBaseFramework` (`self.Parameter`)))))

(fn `GetParameterType`
  (returns (Type :type "/Game/DsQuestAndDialogueSystem/Blueprints/Enums/Quest/Enum_DSsQuestParameterType Enum"))
  (bind (_parameter_description _parameter_correspondinguniqueparameterids _parameter_type) (break `/Game/DsQuestAndDialogueSystem/Blueprints/Structs/Quest/Struct_DSsQuestParameterBaseFramework` (`self.Parameter`)))
  (return _parameter_type))

(fn `GetReqValue`
  (returns (RequiredValue :type "Float (double-precision)"))
  (bind (_parameter_description _parameter_correspondinguniqueparameterids _parameter_type _parameter_requiredamount) (break `/Game/DsQuestAndDialogueSystem/Blueprints/Structs/Quest/Struct_DSsQuestParameterBaseFramework` (`self.Parameter`)))
  (return _parameter_requiredamount))

(fn `GetSection`
  (returns (Section :type "/Game/DsQuestAndDialogueSystem/Blueprints/QuestSystem/BP_DSsQuestSectionBase Object Reference"))
  (locals (Empty :type "/Game/DsQuestAndDialogueSystem/Blueprints/QuestSystem/BP_DSsQuestSectionBase Object Reference"))
  (bind _asbp_sos_quest_section_base (cast `/Game/DsQuestAndDialogueSystem/Blueprints/QuestSystem/BP_DSsQuestSectionBase` (`KismetSystemLibrary.GetOuterObject` self))
    (:`then`
      (return _asbp_sos_quest_section_base))
    (:`CastFailed`
      (return (`local.Empty`)))))

(fn `GetStatus`
  (returns (Status :type "/Game/DsQuestAndDialogueSystem/Blueprints/Enums/Quest/Enum_DSsQuestParameterStatus Enum"))
  (bind (_parameter_description _parameter_correspondinguniqueparameterids _parameter_type _parameter_requiredamount _parameter_hidden _parameter_status) (break `/Game/DsQuestAndDialogueSystem/Blueprints/Structs/Quest/Struct_DSsQuestParameterBaseFramework` (`self.Parameter`)))
  (return _parameter_status))

(fn `GetType`
  (returns (Type :type "/Game/DsQuestAndDialogueSystem/Blueprints/Enums/Quest/Enum_DSsQuestParameterType Enum"))
  (return (`.Type_25_0A1373B24C8FC880CE387DAFC501FE52` (break `/Game/DsQuestAndDialogueSystem/Blueprints/Structs/Quest/Struct_DSsQuestParameterBaseFramework` (`self.Parameter`)))))

(fn `Increment`
  (params (Fragment :type "/Game/DsQuestAndDialogueSystem/Blueprints/Structs/Quest/Struct_DSsQuestFragment Structure"))
  (returns (Output :type Boolean))
  (bind (_type _id _value) (break `/Game/DsQuestAndDialogueSystem/Blueprints/Structs/Quest/Struct_DSsQuestFragment` Fragment))
  (bind (_parameter_description _parameter_correspondinguniqueparameterids _parameter_type _parameter_requiredamount) (break `/Game/DsQuestAndDialogueSystem/Blueprints/Structs/Quest/Struct_DSsQuestParameterBaseFramework` (`self.Parameter`)))
  (bind (_description _correspondinguniqueparameterids _type_2 _requiredamount) (break `/Game/DsQuestAndDialogueSystem/Blueprints/Structs/Quest/Struct_DSsQuestParameterBaseFramework` (`self.Parameter`)))
  (if (`self.CheckID` _id)
    (if (< (`self.CurrentValue`) _parameter_requiredamount)
      (set `self.IsCompleted` false)
      (set `self.CurrentValue` (+ (`self.CurrentValue`) _value))
      (if (< (`self.CurrentValue`) 0.0)
        (set `self.CurrentValue` 0.0))
      (if (>= (`self.CurrentValue`) _requiredamount)
        (set `self.CurrentValue` _requiredamount)
        (set `self.IsCompleted` true)
        (return true)
        (else
          (return true)))
      (elif (< _value 0.0)
        (set `self.IsCompleted` false)
        (set `self.CurrentValue` (+ (`self.CurrentValue`) _value))
        (if (< (`self.CurrentValue`) 0.0)
          (set `self.CurrentValue` 0.0))
        (if (>= (`self.CurrentValue`) _requiredamount)
          (set `self.CurrentValue` _requiredamount)
          (set `self.IsCompleted` true)
          (return true)
          (else
            (return true)))
        (else
          (return false))))
    (else
      (return false))))

(fn `IncrementByItem`
  (params (Item :type "/Game/DsQuestAndDialogueSystem/Blueprints/FrameworkOnly/BP_DSsItemInfo Object Reference"))
  (returns (Output :type Boolean))
  (bind (_parameter_description _parameter_correspondinguniqueparameterids _parameter_type _parameter_requiredamount) (break `/Game/DsQuestAndDialogueSystem/Blueprints/Structs/Quest/Struct_DSsQuestParameterBaseFramework` (`self.Parameter`)))
  (bind (_description _correspondinguniqueparameterids _type _requiredamount) (break `/Game/DsQuestAndDialogueSystem/Blueprints/Structs/Quest/Struct_DSsQuestParameterBaseFramework` (`self.Parameter`)))
  (bind (_type_2 _id _value) (break `/Game/DsQuestAndDialogueSystem/Blueprints/Structs/Quest/Struct_DSsQuestFragment` (`.QuestFragment_22_94AE95B24814A21B53FA7A899A100156` (break `/Game/DsQuestAndDialogueSystem/Blueprints/Structs/Framework/Struct_DSsItemInfoBase` (`/Game/DsQuestAndDialogueSystem/Blueprints/FrameworkOnly/BP_DSsItemInfo.ItemInfo` Item)))))
  (if (`self.CheckID` _id)
    (if (< (`self.CurrentValue`) _parameter_requiredamount)
      (set `self.IsCompleted` false)
      (set `self.CurrentValue` (+ (`self.CurrentValue`) _value))
      (if (< (`self.CurrentValue`) 0.0)
        (set `self.CurrentValue` 0.0))
      (if (>= (`self.CurrentValue`) _requiredamount)
        (set `self.CurrentValue` _requiredamount)
        (set `self.IsCompleted` true)
        (return true)
        (else
          (return true)))
      (elif (< _value 0.0)
        (set `self.IsCompleted` false)
        (set `self.CurrentValue` (+ (`self.CurrentValue`) _value))
        (if (< (`self.CurrentValue`) 0.0)
          (set `self.CurrentValue` 0.0))
        (if (>= (`self.CurrentValue`) _requiredamount)
          (set `self.CurrentValue` _requiredamount)
          (set `self.IsCompleted` true)
          (return true)
          (else
            (return true)))
        (else
          (return false))))
    (else
      (return false))))

(fn `IsEnabled`
  (returns (Enabled :type Boolean))
  (bind (_parameter_description _parameter_correspondinguniqueparameterids _parameter_type _parameter_requiredamount _parameter_hidden _parameter_status) (break `/Game/DsQuestAndDialogueSystem/Blueprints/Structs/Quest/Struct_DSsQuestParameterBaseFramework` (`self.Parameter`)))
  (if (or (`|EnumEquality` _parameter_status "NewEnumerator3") (`|EnumEquality` _parameter_status "NewEnumerator7") (`|EnumEquality` _parameter_status "NewEnumerator8"))
    (return true)
    (else
      (return false))))

(fn `IsFragmentValid `
  (params (ID :type String))
  (returns (Return :type Boolean))
  (return (`KismetArrayLibrary.Array_Contains` (`.CorrespondingUniqueParameterIDs_14_03DD5036465675D42860EA8589D17ED8` (break `/Game/DsQuestAndDialogueSystem/Blueprints/Structs/Quest/Struct_DSsQuestParameterBaseFramework` (`self.Parameter`))) ID)))

(fn `IsHidden`
  (returns (Hidden :type Boolean))
  (bind (_parameter_description _parameter_correspondinguniqueparameterids _parameter_type _parameter_requiredamount _parameter_hidden) (break `/Game/DsQuestAndDialogueSystem/Blueprints/Structs/Quest/Struct_DSsQuestParameterBaseFramework` (`self.Parameter`)))
  (return _parameter_hidden))

(fn `IsReqCompleted`
  (returns (Return :type Boolean))
  (return (>= (`self.CurrentValue`) (`.RequiredAmount_41_289429B5464A19ED43DB2593B832DFC4` (break `/Game/DsQuestAndDialogueSystem/Blueprints/Structs/Quest/Struct_DSsQuestParameterBaseFramework` (`self.Parameter`))))))

(fn `ParameterUpdated_CallBack`
  (params (Reason :type "/Game/DsQuestAndDialogueSystem/Blueprints/Enums/Quest/Enum_DSsQuestSectionParameterUpdateReason Enum" :default "NewEnumerator4"))
  (`self.ParameterUpdated` self Reason))

(fn `SetParameterDescription`
  (params (Description :type String))
  (bind (_description _correspondinguniqueparameterids _type _requiredamount _hidden _status) (break `/Game/DsQuestAndDialogueSystem/Blueprints/Structs/Quest/Struct_DSsQuestParameterBaseFramework` (`self.Parameter`)))
  (set `self.Parameter` (make `/Game/DsQuestAndDialogueSystem/Blueprints/Structs/Quest/Struct_DSsQuestParameterBaseFramework` Description _correspondinguniqueparameterids _type _requiredamount _hidden _status)))

(fn `SetStatus`
  (params (Status :type "/Game/DsQuestAndDialogueSystem/Blueprints/Enums/Quest/Enum_DSsQuestParameterStatus Enum" :default "NewEnumerator3"))
  (bind (_description _correspondinguniqueparameterids _type _requiredamount _hidden _status) (break `/Game/DsQuestAndDialogueSystem/Blueprints/Structs/Quest/Struct_DSsQuestParameterBaseFramework` (`self.Parameter`)))
  (if (!= Status _status)
    (set `self.Parameter` (make `/Game/DsQuestAndDialogueSystem/Blueprints/Structs/Quest/Struct_DSsQuestParameterBaseFramework` _description _correspondinguniqueparameterids _type _requiredamount _hidden Status))
    (`self.ParameterUpdated` self "NewEnumerator1")))

(fn `SetVisibility`
  (params (Hidden :type Boolean))
  (bind (_parameter_description _parameter_correspondinguniqueparameterids _parameter_type _parameter_requiredamount _parameter_hidden _parameter_status) (break `/Game/DsQuestAndDialogueSystem/Blueprints/Structs/Quest/Struct_DSsQuestParameterBaseFramework` (`self.Parameter`)))
  (set `self.Parameter` (make `/Game/DsQuestAndDialogueSystem/Blueprints/Structs/Quest/Struct_DSsQuestParameterBaseFramework` _parameter_description _parameter_correspondinguniqueparameterids _parameter_type _parameter_requiredamount Hidden _parameter_status))
  (`self.ParameterUpdated` self "NewEnumerator1"))

(fn `ToString`
  (returns (return :type String))
  (bind (_parameter_description _parameter_correspondinguniqueparameterids _parameter_type _parameter_requiredamount) (break `/Game/DsQuestAndDialogueSystem/Blueprints/Structs/Quest/Struct_DSsQuestParameterBaseFramework` (`self.Parameter`)))
  ;[1 1 1] Get Parameter string according to type of parameter
  (switch `/Game/DsQuestAndDialogueSystem/Blueprints/Enums/Quest/Enum_DSsQuestParameterType` _parameter_type
    (:`NewEnumerator3`
      (return ""))
    (:`NewEnumerator4`
      (return (`KismetStringLibrary.Concat_StrStr` _parameter_description " : " (`KismetStringLibrary.Conv_IntToString` (`KismetMathLibrary.Round` (`self.CurrentValue`))) "/" (`KismetStringLibrary.Conv_IntToString` (`KismetMathLibrary.Round` _parameter_requiredamount)))))
    (:`NewEnumerator5`
      (return (`KismetStringLibrary.Concat_StrStr` _parameter_description " : " (`KismetStringLibrary.Conv_DoubleToString` (`self.CurrentValue`)) "/" (`KismetStringLibrary.Conv_DoubleToString` _parameter_requiredamount))))
    (:`NewEnumerator6`
      (return _parameter_description))))
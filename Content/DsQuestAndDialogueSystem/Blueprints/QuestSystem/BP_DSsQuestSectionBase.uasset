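; Quest section object that groups a quest's parameters (objectives) and tracks the section's status and visibility.
; It builds parameter objects from the section struct and relays their updates.
; Fragments or items advance enabled parameters, completing the section when all requirements are met; fragment-driven completion also runs trigger scripts through the quest manager.
; Counted items are recorded so their removal rolls back progress, and can later be consumed.
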(fn `AddParameter`
  (params (NewParamter :type "/Game/DsQuestAndDialogueSystem/Blueprints/Structs/Quest/Struct_DSsQuestParameterBaseFramework Structure") (Index :type Integer :default 0))
  (bind _returnvalue (`|GenericCreateObject` self "/Game/DsQuestAndDialogueSystem/Blueprints/QuestSystem/BP_DSsQuestParameterBase.BP_DSsQuestParameterBase_C" NewParamter))
  (`KismetArrayLibrary.Array_Insert` (`self.Parameters`) _returnvalue Index)
  (add `/Game/DsQuestAndDialogueSystem/Blueprints/QuestSystem/BP_DSsQuestParameterBase.ParameterUpdated` _returnvalue (`|CreateDelegate` :!event `ParameterUpdated_callback`))
  (`self.SectionUpdated` self "NewEnumerator9"))

(fn `CallNextParameter`
  (params (Parameter :type "/Game/DsQuestAndDialogueSystem/Blueprints/QuestSystem/BP_DSsQuestParameterBase Object Reference (by ref)"))
  (bind _parameters (`self.Parameters`))
  (bind _returnvalue (+ (`KismetArrayLibrary.Array_Find` _parameters Parameter) 1))
  (bind _output (`|GetArrayItem` _parameters _returnvalue))
  ;[1 1 1] If parameter is hidden after completed call next parameter
  (if (`KismetArrayLibrary.Array_IsValidIndex` _parameters _returnvalue)
    (`/Engine/EditorBlueprintResources/StandardMacros.IsValid` _output
      (:`Is Valid`
        (if (`|EnumEquality` (`/Game/DsQuestAndDialogueSystem/Blueprints/QuestSystem/BP_DSsQuestParameterBase.GetStatus` _output) "NewEnumerator5")
          (`/Game/DsQuestAndDialogueSystem/Blueprints/QuestSystem/BP_DSsQuestParameterBase.SetStatus` _output "NewEnumerator3"))))))

(fn `CallNextSection`
  (`/Game/DsQuestAndDialogueSystem/Blueprints/QuestSystem/BP_DSsQuestBase.CallNextSection` (`self.GetQuest`) self))

(fn `CheckSectionParametersCompleted`
  (returns (Return :type Boolean))
  (locals (Completed :type Boolean))
  (for _array_element (`self.Parameters`)
    (if (`/Game/DsQuestAndDialogueSystem/Blueprints/QuestSystem/BP_DSsQuestParameterBase.IsReqCompleted` _array_element)
      (set `local.Completed` true)
      (else
        (return false))))
  (if (`local.Completed`)
    (return (`local.Completed`))
    (else
      (return false))))

(fn `ConsumeRecordedItems`
  ;[1 0 0] Determine whether recorded quest item will be removed or not. If quest item value less than current parameter value it will be consumed and removed.
  (for _array_element (`self.Parameters`)
    (for _array_element_2 (`self.RecordedItems`)
      (`/Game/DsQuestAndDialogueSystem/Blueprints/QuestSystem/BP_DSsQuestParameterBase.ConsumeItem` _array_element _array_element_2)
      (`/Game/DsQuestAndDialogueSystem/Blueprints/FrameworkOnly/BP_DSsItemInfo.ToBeRemoved` _array_element_2 _array_element_2))))

(fn `DecrementParameters`
  (params (ItemInfo :type "/Game/DsQuestAndDialogueSystem/Blueprints/FrameworkOnly/BP_DSsItemInfo Object Reference"))
  ;[1 1 1] When item is removed, the item value will drop from the parameter value.
  (if (`|EnumEquality` (`/Game/DsQuestAndDialogueSystem/Blueprints/QuestSystem/BP_DSsQuestBase.QuestProgress` (`self.GetQuest`)) "NewEnumerator0")
    (if (`KismetArrayLibrary.Array_Contains` (`self.RecordedItems`) ItemInfo)
      (for _array_element (`self.Parameters`)
        (bind _return (`/Game/DsQuestAndDialogueSystem/Blueprints/QuestSystem/BP_DSsQuestParameterBase.DecrementByItem` _array_element ItemInfo))
        (if (and _return (`/Game/DsQuestAndDialogueSystem/Blueprints/FrameworkOnly/BP_DSsItemInfo.IsFragmentConsumed` ItemInfo))
          (`KismetArrayLibrary.Array_RemoveItem` (`self.RecordedItems`) ItemInfo)
          (else
            (`KismetArrayLibrary.Array_RemoveItem` (`self.RecordedItems`) ItemInfo)
            (`self.ProgressSectionByItem` ItemInfo))))
      (`self.ScanInventoryForNewItems`)
      (if (`self.CheckSectionParametersCompleted`)
        (`self.SetSectionStatus` "NewEnumerator7")
        (else
          (`self.SetSectionStatus` "NewEnumerator3"))))))

(fn `DoesItNeedToBeRemoved`
  (returns (Return :type Boolean))
  (bind (_id _sectionstatus _hideaftercompletedorfailed) (break `/Game/DsQuestAndDialogueSystem/Blueprints/Structs/Quest/Struct_DSsQuestParameterSectionFramework` (`self.Section`)))
  (if (or (`|EnumEquality` _sectionstatus "NewEnumerator4") (`|EnumEquality` _sectionstatus "NewEnumerator5"))
    (return true)
    (elif (and _hideaftercompletedorfailed (or (`|EnumEquality` _sectionstatus "NewEnumerator7") (`|EnumEquality` _sectionstatus "NewEnumerator8")))
      (return true)
      (else
        (return false)))))

(fn `ForceCompleteSection`
  (`self.SetSectionStatus` "NewEnumerator7")
  (for _array_element (`self.Parameters`)
    (`/Game/DsQuestAndDialogueSystem/Blueprints/QuestSystem/BP_DSsQuestParameterBase.ForceCompleteParameter` _array_element))
  (`self.SectionUpdated` self "NewEnumerator6"))

(fn `GetID`
  (returns (`Section ID` :type String))
  (bind _section_id (break `/Game/DsQuestAndDialogueSystem/Blueprints/Structs/Quest/Struct_DSsQuestParameterSectionFramework` (`self.Section`)))
  (return _section_id))

(fn `GetLastAddedParameter`
  (returns (Output :type "/Game/DsQuestAndDialogueSystem/Blueprints/QuestSystem/BP_DSsQuestParameterBase Object Reference"))
  (locals (Empty :type "/Game/DsQuestAndDialogueSystem/Blueprints/QuestSystem/BP_DSsQuestParameterBase Object Reference"))
  (bind _parameters (`self.Parameters`))
  (bind _output (`|GetArrayItem` _parameters (- (`KismetArrayLibrary.Array_Length` _parameters) 1)))
  (`/Engine/EditorBlueprintResources/StandardMacros.IsValid` _output
    (:`Is Valid`
      (return _output))
    (:`Is Not Valid`
      (return (`local.Empty`)))))

(fn `GetParameter`
  (params (Index :type Integer))
  (returns (Output :type "/Game/DsQuestAndDialogueSystem/Blueprints/QuestSystem/BP_DSsQuestParameterBase Object Reference"))
  (return (`|GetArrayItem` (`self.Parameters`) Index)))

(fn `GetParameters`
  (returns (Parameters :type "Array of /Game/DsQuestAndDialogueSystem/Blueprints/QuestSystem/BP_DSsQuestParameterBase Object Reference"))
  (return (`self.Parameters`)))

(fn `GetParameterSize`
  (returns (Return :type Integer))
  (return (`KismetArrayLibrary.Array_Length` (`self.Parameters`))))

(fn `GetQuest`
  (returns (`AsQuest Base` :type "/Game/DsQuestAndDialogueSystem/Blueprints/QuestSystem/BP_DSsQuestBase Object Reference"))
  (locals (Empty :type "/Game/DsQuestAndDialogueSystem/Blueprints/QuestSystem/BP_DSsQuestBase Object Reference"))
  (bind _asbp_sos_quest_base (cast `/Game/DsQuestAndDialogueSystem/Blueprints/QuestSystem/BP_DSsQuestBase` (`KismetSystemLibrary.GetOuterObject` self))
    (:`then`
      (return _asbp_sos_quest_base))
    (:`CastFailed`
      (return (`local.Empty`)))))

(fn `GetSectionStatus`
  (returns (`Section Section Status` :type "/Game/DsQuestAndDialogueSystem/Blueprints/Enums/Quest/Enum_DSsQuestParameterSectionStatus Enum"))
  (bind (_section_id _section_sectionstatus) (break `/Game/DsQuestAndDialogueSystem/Blueprints/Structs/Quest/Struct_DSsQuestParameterSectionFramework` (`self.Section`)))
  (return _section_sectionstatus))

(fn `IsSectionActive`
  (returns (Return :type Boolean))
  (return (`|EnumEquality` (`self.GetSectionStatus`) "NewEnumerator3")))

(fn `IsSectionCompleted`
  (returns (IsCompleted :type Boolean))
  (bind (_section_id _section_sectionstatus) (break `/Game/DsQuestAndDialogueSystem/Blueprints/Structs/Quest/Struct_DSsQuestParameterSectionFramework` (`self.Section`)))
  (return (`|EnumEquality` _section_sectionstatus "NewEnumerator7")))

(fn `IsSectionEnabled`
  (returns (Return :type Boolean))
  (bind (_id _sectionstatus _hideaftercompletedorfailed) (break `/Game/DsQuestAndDialogueSystem/Blueprints/Structs/Quest/Struct_DSsQuestParameterSectionFramework` (`self.Section`)))
  (if (or (`|EnumEquality` _sectionstatus "NewEnumerator4") (`|EnumEquality` _sectionstatus "NewEnumerator5"))
    (return false)
    (elif (and _hideaftercompletedorfailed (or (`|EnumEquality` _sectionstatus "NewEnumerator7") (`|EnumEquality` _sectionstatus "NewEnumerator8")))
      (return false)
      (else
        (return true)))))

(fn `OnCreate`
  (for _array_element (`.Parameters_5_E67824284B5E4D1FE6D0E7B3C7FE2C8A` (break `/Game/DsQuestAndDialogueSystem/Blueprints/Structs/Quest/Struct_DSsQuestParameterSectionFramework` (`self.Section`)))
    (bind _returnvalue (`|GenericCreateObject` self "/Game/DsQuestAndDialogueSystem/Blueprints/QuestSystem/BP_DSsQuestParameterBase.BP_DSsQuestParameterBase_C" _array_element))
    (`KismetArrayLibrary.Array_Add` (`self.Parameters`) _returnvalue)
    (add `/Game/DsQuestAndDialogueSystem/Blueprints/QuestSystem/BP_DSsQuestParameterBase.ParameterUpdated` _returnvalue (`|CreateDelegate` :!event `ParameterUpdated_callback`))
    (`self.SectionUpdated` self "NewEnumerator9"))
  (`self.SectionUpdated` self "NewEnumerator6"))

(fn `ParametersToString`
  (returns (return :type "Array of String"))
  (locals (String :type "Array of String"))
  (for _array_element (`self.Parameters`)
    (`KismetArrayLibrary.Array_Add` (`local.String`) (`/Game/DsQuestAndDialogueSystem/Blueprints/QuestSystem/BP_DSsQuestParameterBase.ToString` _array_element)))
  (return (`local.String`)))

(fn `ParameterUpdated_callback`
  (params (Parameter :type "/Game/DsQuestAndDialogueSystem/Blueprints/QuestSystem/BP_DSsQuestParameterBase Object Reference") (Reason :type "/Game/DsQuestAndDialogueSystem/Blueprints/Enums/Quest/Enum_DSsQuestSectionParameterUpdateReason Enum" :default "NewEnumerator4"))
  (`self.ParameterUpdated` Parameter Reason))

(fn `ProgressSection`
  (params (Fragment :type "/Game/DsQuestAndDialogueSystem/Blueprints/Structs/Quest/Struct_DSsQuestFragment Structure"))
  ;[1 1 1] If Parameter enabled then progress.
  (for _array_element (`self.Parameters`)
    (if (`/Game/DsQuestAndDialogueSystem/Blueprints/QuestSystem/BP_DSsQuestParameterBase.IsEnabled` _array_element)
      (bind _output (`/Game/DsQuestAndDialogueSystem/Blueprints/QuestSystem/BP_DSsQuestParameterBase.Increment` _array_element Fragment))
      (if _output
        (`self.ParameterUpdated_callback` _array_element (select `bool` (`/Game/DsQuestAndDialogueSystem/Blueprints/QuestSystem/BP_DSsQuestParameterBase.GetIsCompleted` _array_element) :`false` "NewEnumerator0" :`true` (select `bool` (`/Game/DsQuestAndDialogueSystem/Blueprints/QuestSystem/BP_DSsQuestParameterBase.GetIsFailed` _array_element) :`false` "NewEnumerator2" :`true` "NewEnumerator8" :!type "/Game/DsQuestAndDialogueSystem/Blueprints/Enums/Quest/Enum_DSsQuestSectionParameterUpdateReason Enum"))))))
  (if (`self.CheckSectionParametersCompleted`)
    (`self.SetSectionStatus` "NewEnumerator7")
    (`self.SectionUpdated` self "NewEnumerator6")
    (`/Game/DsQuestAndDialogueSystem/Blueprints/QuestSystem/BP_DSsQuestManager_Component.RunScripts` (`/Game/DsQuestAndDialogueSystem/Blueprints/QuestSystem/BP_DSsQuestBase.GetQuestManager` (`self.GetQuest`)) (`.SectionCompletedTrigger_24_A8BEB803457E14FE0540C2BDB1EAC20A` (break `/Game/DsQuestAndDialogueSystem/Blueprints/Structs/Quest/Struct_DSsQuestParameterSectionFramework` (`self.Section`))))
    (else
      (`self.SectionUpdated` self "NewEnumerator6"))))

(fn `ProgressSectionByItem`
  (params (Item :type "/Game/DsQuestAndDialogueSystem/Blueprints/FrameworkOnly/BP_DSsItemInfo Object Reference"))
  ;[1 1 1] If Parameter enabled then progress and record that item.
  (for _array_element (`self.Parameters`)
    (if (`/Game/DsQuestAndDialogueSystem/Blueprints/QuestSystem/BP_DSsQuestParameterBase.IsEnabled` _array_element)
      (if (not (`KismetArrayLibrary.Array_Contains` (`self.RecordedItems`) Item))
        (bind _output (`/Game/DsQuestAndDialogueSystem/Blueprints/QuestSystem/BP_DSsQuestParameterBase.IncrementByItem` _array_element Item))
        (if _output
          (`self.ParameterUpdated_callback` _array_element (select `bool` (`/Game/DsQuestAndDialogueSystem/Blueprints/QuestSystem/BP_DSsQuestParameterBase.GetIsCompleted` _array_element) :`false` "NewEnumerator0" :`true` (select `bool` (`/Game/DsQuestAndDialogueSystem/Blueprints/QuestSystem/BP_DSsQuestParameterBase.GetIsFailed` _array_element) :`false` "NewEnumerator2" :`true` "NewEnumerator8" :!type "/Game/DsQuestAndDialogueSystem/Blueprints/Enums/Quest/Enum_DSsQuestSectionParameterUpdateReason Enum")))
          ;;[1 0 0] When this item is removed, the item value will drop from the parameter value.
          (`KismetArrayLibrary.Array_Add` (`self.RecordedItems`) Item)
          (add `/Game/DsQuestAndDialogueSystem/Blueprints/FrameworkOnly/BP_DSsItemInfo.ToBeRemoved` Item (`|CreateDelegate` :!event `DecrementParameters`))))))
  (if (`self.CheckSectionParametersCompleted`)
    (`self.SetSectionStatus` "NewEnumerator7")
    (`self.SectionUpdated` self "NewEnumerator6")
    (else
      (`self.SectionUpdated` self "NewEnumerator6"))))

(fn `RemoveParameter`
  (params (ID :type "/Game/DsQuestAndDialogueSystem/Blueprints/Structs/Quest/Struct_DSsQuestParameterID Structure"))
  (`KismetArrayLibrary.Array_Remove` (`self.Parameters`) ID_Parameter_7_7BCCB6234EAE1D271D956A9CCB13BB8C)
  (`self.SectionUpdated` self "NewEnumerator10"))

(fn `SetSectionStatus`
  (params (Status :type "/Game/DsQuestAndDialogueSystem/Blueprints/Enums/Quest/Enum_DSsQuestParameterSectionStatus Enum" :default "NewEnumerator3"))
  (locals (VisibilityUpdated :type Boolean))
  (bind (_id _sectionstatus _hideaftercompletedorfailed _sectioncompletedtrigger _parameters) (break `/Game/DsQuestAndDialogueSystem/Blueprints/Structs/Quest/Struct_DSsQuestParameterSectionFramework` (`self.Section`)))
  (if (!= Status _sectionstatus)
    (if (or (and (`|EnumEquality` _sectionstatus "NewEnumerator3") (`|EnumEquality` Status "NewEnumerator4")) (and (`|EnumEquality` _sectionstatus "NewEnumerator4") (`|EnumEquality` Status "NewEnumerator3")) (and (`|EnumEquality` _sectionstatus "NewEnumerator5") (`|EnumEquality` Status "NewEnumerator3")) (and (`|EnumEquality` Status "NewEnumerator3") (`|EnumEquality` _sectionstatus "NewEnumerator5")) (and (or (and (`|EnumEquality` _sectionstatus "NewEnumerator7") (`|EnumEquality` Status "NewEnumerator3")) (and (`|EnumEquality` _sectionstatus "NewEnumerator8") (`|EnumEquality` Status "NewEnumerator3"))) _hideaftercompletedorfailed) (and _hideaftercompletedorfailed (or (and (`|EnumEquality` _sectionstatus "NewEnumerator3") (`|EnumEquality` Status "NewEnumerator7")) (and (`|EnumEquality` _sectionstatus "NewEnumerator3") (`|EnumEquality` Status "NewEnumerator8")))) (and (`|EnumEquality` Status "NewEnumerator4") (`|EnumEquality` _sectionstatus "NewEnumerator7")) (and (`|EnumEquality` Status "NewEnumerator7") (`|EnumEquality` _sectionstatus "NewEnumerator4")) (and (`|EnumEquality` Status "NewEnumerator8") (`|EnumEquality` _sectionstatus "NewEnumerator4")) (and (`|EnumEquality` Status "NewEnumerator4") (`|EnumEquality` _sectionstatus "NewEnumerator8")))
      (set `local.VisibilityUpdated` true)
      (else
        (set `local.VisibilityUpdated` false)))
    (set `self.Section` (make `/Game/DsQuestAndDialogueSystem/Blueprints/Structs/Quest/Struct_DSsQuestParameterSectionFramework` _id Status _hideaftercompletedorfailed _sectioncompletedtrigger _parameters))
    (if (`local.VisibilityUpdated`)
      (`self.SectionUpdated` self "NewEnumerator7"))))
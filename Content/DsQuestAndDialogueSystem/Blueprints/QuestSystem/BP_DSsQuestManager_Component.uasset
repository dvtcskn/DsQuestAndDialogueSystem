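; Quest manager component that tracks quests through active, completed and failed lists plus a blacklist, with lookup, restart, abandon and removal.
; Quests start from data table rows or structs as BP_DSsQuestBase objects, whose update events are relayed through dispatchers.
; Fragments and items progress active quests bound to them.
; Quest state changes fire signal fragments into other quests, and completion can fail or blacklist listed quests.
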(fn `AbandonQuest`
  (params (Quest :type "DataTableRowHandle Structure"))
  (bind _returnvalue (`|GetDataTableRow` Quest_DataTable Quest_RowName)
    (:`then`
      (bind (_questname _questid) (break `/Game/DsQuestAndDialogueSystem/Blueprints/Structs/Quest/Struct_DSsQuestFramework` _returnvalue))
      (bind _value (`BlueprintMapLibrary.Map_Find` (`self.ActiveQuestList`) _questid))
      (`/Engine/EditorBlueprintResources/StandardMacros.IsValid` _value
        (:`Is Valid`
          (`self.RemovedQuestDispatcher` _value)
          (`BlueprintMapLibrary.Map_Remove` (`self.ActiveQuestList`) _questid))))))

(fn `AbandonQuestByID`
  (params (Quest :type String))
  (bind _value (`BlueprintMapLibrary.Map_Find` (`self.ActiveQuestList`) Quest))
  (`/Engine/EditorBlueprintResources/StandardMacros.IsValid` _value
    (:`Is Valid`
      (`self.RemovedQuestDispatcher` _value)
      (`BlueprintMapLibrary.Map_Remove` (`self.ActiveQuestList`) Quest))))

(fn `AddParameterToQuest`
  (params (ID :type "/Game/DsQuestAndDialogueSystem/Blueprints/Structs/Quest/Struct_DSsQuestParameterID Structure") (Parameter :type "/Game/DsQuestAndDialogueSystem/Blueprints/Structs/Quest/Struct_DSsQuestParameterBaseFramework Structure"))
  (bind _values (`BlueprintMapLibrary.Map_Values` (`self.ActiveQuestList`)))
  (for _array_element _values
    (if (`KismetStringLibrary.EqualEqual_StrStr` (`/Game/DsQuestAndDialogueSystem/Blueprints/QuestSystem/BP_DSsQuestBase.GetQuestID` _array_element) (`.QuestID_10_4834D5E148B1D1234916BE874771298C` (break `/Game/DsQuestAndDialogueSystem/Blueprints/Structs/Quest/Struct_DSsQuestParameterID` ID)))
      (`/Game/DsQuestAndDialogueSystem/Blueprints/QuestSystem/BP_DSsQuestBase.AddParameter` _array_element ID Parameter))))

(fn `AddQuestToBlacklist`
  (params (Quest :type "/Game/DsQuestAndDialogueSystem/Blueprints/Structs/Quest/Struct_DSsQuestFramework Structure (by ref)"))
  (`KismetArrayLibrary.Array_Add` (`self.QuestBlackList`) Quest)
  (for _array_element (`.SignalOtherQuests_47_7E84C6434609FBE9249F6DB01217D9BB` (break `/Game/DsQuestAndDialogueSystem/Blueprints/Structs/Quest/Struct_DSsQuestFramework` Quest))
    (bind (_state _fragment) (break `/Game/DsQuestAndDialogueSystem/Blueprints/Structs/Quest/Struct_DSsQuestSignalFragment` _array_element))
    (if (`|EnumEquality` _state "NewEnumerator3")
      (`self.ProgressQuest` _fragment))))

(fn `CompletedQuest`
  (params (Quest :type "/Game/DsQuestAndDialogueSystem/Blueprints/QuestSystem/BP_DSsQuestBase Object Reference"))
  (bind _id (`/Game/DsQuestAndDialogueSystem/Blueprints/QuestSystem/BP_DSsQuestBase.GetID` Quest))
  (bind (_questname _questid _questdescription _queststartscripts _questendscripts _parametersections _rewards _queststofailorblacklist _signalotherquests) (break `/Game/DsQuestAndDialogueSystem/Blueprints/Structs/Quest/Struct_DSsQuestFramework` (`/Game/DsQuestAndDialogueSystem/Blueprints/QuestSystem/BP_DSsQuestBase.QuestBase` Quest)))
  (`BlueprintMapLibrary.Map_Add` (`self.CompletedQuestList`) _id Quest)
  (`BlueprintMapLibrary.Map_Remove` (`self.ActiveQuestList`) _id)
  (`self.CompletedQuestDispatcher` Quest)
  ;[0 0 0] AfterCompleted Fail or add black list Selected quests
  (for _array_element _queststofailorblacklist
    (bind (_datatable _rowname) (break `DataTableRowHandle` _array_element))
    (if (and (`KismetSystemLibrary.IsValid` _datatable) (!= _rowname "None"))
      (bind _returnvalue (`|GetDataTableRow` _datatable _rowname)
        (:`then`
          (bind _quest (`self.GetQuestByID` "NewEnumerator0" (`.QuestID_4_4DA48B5A4D4871FBE8DA14A70DAE74DD` (break `/Game/DsQuestAndDialogueSystem/Blueprints/Structs/Quest/Struct_DSsQuestFramework` _returnvalue))))
          (`/Engine/EditorBlueprintResources/StandardMacros.IsValid` _quest
            (:`Is Valid`
              (`/Game/DsQuestAndDialogueSystem/Blueprints/QuestSystem/BP_DSsQuestBase.ForceFailQuest` _quest))
            (:`Is Not Valid`
              (`self.AddQuestToBlacklist` _returnvalue)))))))
  (for _array_element_2 _signalotherquests
    (bind (_state _fragment) (break `/Game/DsQuestAndDialogueSystem/Blueprints/Structs/Quest/Struct_DSsQuestSignalFragment` _array_element_2))
    (switch `/Game/DsQuestAndDialogueSystem/Blueprints/Enums/Quest/Enum_DSsQuestSignalState` _state
      (:`NewEnumerator1`
        (`self.ProgressQuest` _fragment)))))

(fn `CompleteQuest`
  (params (ID :type String))
  (bind _quest (`self.GetQuestByID` "NewEnumerator0" ID))
  (`/Engine/EditorBlueprintResources/StandardMacros.IsValid` _quest
    (:`Is Valid`
      (if (`/Game/DsQuestAndDialogueSystem/Blueprints/QuestSystem/BP_DSsQuestBase.CheckQuestReqCompleted` _quest)
        (`/Game/DsQuestAndDialogueSystem/Blueprints/QuestSystem/BP_DSsQuestBase.CompleteQuest` _quest)))))

(fn `CreateQuest`
  (params (InQuest :type "/Game/DsQuestAndDialogueSystem/Blueprints/Structs/Quest/Struct_DSsQuestFramework Structure"))
  (locals (ID :type String) (Temp :type "/Game/DsQuestAndDialogueSystem/Blueprints/QuestSystem/BP_DSsQuestBase Object Reference"))
  (bind _returnvalue (`|GenericCreateObject` self "/Game/DsQuestAndDialogueSystem/Blueprints/QuestSystem/BP_DSsQuestBase.BP_DSsQuestBase_C" InQuest))
  (set `local.Temp` _returnvalue)
  (set `local.ID` (`/Game/DsQuestAndDialogueSystem/Blueprints/QuestSystem/BP_DSsQuestBase.GetQuestID` _returnvalue))
  (bind _keys (`BlueprintMapLibrary.Map_Keys` (`self.ActiveQuestList`)))
  (if (not (`KismetArrayLibrary.Array_Contains` _keys (`local.ID`)))
    (`BlueprintMapLibrary.Map_Add` (`self.ActiveQuestList`) (`local.ID`) (`local.Temp`))
    (add `/Game/DsQuestAndDialogueSystem/Blueprints/QuestSystem/BP_DSsQuestBase.ScanInventoryForNewItems` (`local.Temp`) (`|CreateDelegate` :!event `ScanInventoryForNewItems_CallBack`))
    (add `/Game/DsQuestAndDialogueSystem/Blueprints/QuestSystem/BP_DSsQuestBase.SectionUpdated` (`local.Temp`) (`|CreateDelegate` :!event `SectionUpdated_Callback`))
    (add `/Game/DsQuestAndDialogueSystem/Blueprints/QuestSystem/BP_DSsQuestBase.ParameterUpdated` (`local.Temp`) (`|CreateDelegate` :!event `ParameterUpdated_Callback`))
    (`/Game/DsQuestAndDialogueSystem/Blueprints/QuestSystem/BP_DSsQuestBase.OnCreate` (`local.Temp`))
    (`self.AddQuestDispatcher` (`local.Temp`))
    ;[1 1 1] Signal Other Quests
    (for _array_element (`.SignalOtherQuests_47_7E84C6434609FBE9249F6DB01217D9BB` (break `/Game/DsQuestAndDialogueSystem/Blueprints/Structs/Quest/Struct_DSsQuestFramework` (`/Game/DsQuestAndDialogueSystem/Blueprints/QuestSystem/BP_DSsQuestBase.QuestBase` (`local.Temp`))))
      (bind (_state _fragment) (break `/Game/DsQuestAndDialogueSystem/Blueprints/Structs/Quest/Struct_DSsQuestSignalFragment` _array_element))
      (if (`|EnumEquality` _state "NewEnumerator0")
        (`self.ProgressQuest` _fragment)))))

(fn `FailedQuest`
  (params (InQuest :type "/Game/DsQuestAndDialogueSystem/Blueprints/QuestSystem/BP_DSsQuestBase Object Reference"))
  (bind _id (`/Game/DsQuestAndDialogueSystem/Blueprints/QuestSystem/BP_DSsQuestBase.GetID` InQuest))
  (`BlueprintMapLibrary.Map_Add` (`self.FailedQuestList`) _id InQuest)
  (`BlueprintMapLibrary.Map_Remove` (`self.ActiveQuestList`) _id)
  (`self.FailedQuestDispatcher` InQuest)
  (for _array_element (`.SignalOtherQuests_47_7E84C6434609FBE9249F6DB01217D9BB` (break `/Game/DsQuestAndDialogueSystem/Blueprints/Structs/Quest/Struct_DSsQuestFramework` (`/Game/DsQuestAndDialogueSystem/Blueprints/QuestSystem/BP_DSsQuestBase.QuestBase` InQuest)))
    (bind (_state _fragment) (break `/Game/DsQuestAndDialogueSystem/Blueprints/Structs/Quest/Struct_DSsQuestSignalFragment` _array_element))
    (if (`|EnumEquality` _state "NewEnumerator2")
      (`self.ProgressQuest` _fragment))))

(fn `ForceCompleteQuest`
  (params (ID :type String))
  (bind _quest (`self.GetQuestByID` "NewEnumerator0" ID))
  (`/Engine/EditorBlueprintResources/StandardMacros.IsValid` _quest
    (:`Is Valid`
      (`/Game/DsQuestAndDialogueSystem/Blueprints/QuestSystem/BP_DSsQuestBase.ForceCompleteQuest` _quest))))

(fn `ForceFailQuest`
  (params (InQuest :type "/Game/DsQuestAndDialogueSystem/Blueprints/QuestSystem/BP_DSsQuestBase Object Reference"))
  (`/Game/DsQuestAndDialogueSystem/Blueprints/QuestSystem/BP_DSsQuestBase.ForceFailQuest` InQuest))

(fn `GetQuestByID`
  (params (Progress :type "/Game/DsQuestAndDialogueSystem/Blueprints/Enums/Quest/Enum_DSsQuestProgression Enum" :default "NewEnumerator0") (ID :type String))
  (returns (Quest :type "/Game/DsQuestAndDialogueSystem/Blueprints/QuestSystem/BP_DSsQuestBase Object Reference"))
  (locals (Empty :type "/Game/DsQuestAndDialogueSystem/Blueprints/QuestSystem/BP_DSsQuestBase Object Reference"))
  (switch `/Game/DsQuestAndDialogueSystem/Blueprints/Enums/Quest/Enum_DSsQuestProgression` Progress
    (:`NewEnumerator0`
      (bind _values (`BlueprintMapLibrary.Map_Values` (`self.ActiveQuestList`)))
      (for _array_element _values
        (if (`KismetStringLibrary.EqualEqual_StrStr` (`/Game/DsQuestAndDialogueSystem/Blueprints/QuestSystem/BP_DSsQuestBase.GetID` _array_element) ID)
          (return _array_element)))
      (return (`local.Empty`)))
    (:`NewEnumerator1`
      (bind _values_2 (`BlueprintMapLibrary.Map_Values` (`self.CompletedQuestList`)))
      (for _array_element_2 _values_2
        (if (`KismetStringLibrary.EqualEqual_StrStr` (`/Game/DsQuestAndDialogueSystem/Blueprints/QuestSystem/BP_DSsQuestBase.GetID` _array_element_2) ID)
          (return _array_element_2)))
      (return (`local.Empty`)))
    (:`NewEnumerator2`
      (bind _values_3 (`BlueprintMapLibrary.Map_Values` (`self.FailedQuestList`)))
      (for _array_element_3 _values_3
        (if (`KismetStringLibrary.EqualEqual_StrStr` (`/Game/DsQuestAndDialogueSystem/Blueprints/QuestSystem/BP_DSsQuestBase.GetID` _array_element_3) ID)
          (return _array_element_3)))
      (return (`local.Empty`)))
    (:`NewEnumerator3`
      (return (`local.Empty`)))))

(fn `GetQuestByIDEx`
  (params (ID :type String))
  (returns (Quest :type "/Game/DsQuestAndDialogueSystem/Blueprints/QuestSystem/BP_DSsQuestBase Object Reference"))
  (locals (Empty :type "/Game/DsQuestAndDialogueSystem/Blueprints/QuestSystem/BP_DSsQuestBase Object Reference"))
  (bind _values (`BlueprintMapLibrary.Map_Values` (`self.ActiveQuestList`)))
  (for _array_element _values
    (if (`KismetStringLibrary.EqualEqual_StrStr` (`/Game/DsQuestAndDialogueSystem/Blueprints/QuestSystem/BP_DSsQuestBase.GetID` _array_element) ID)
      (return _array_element)))
  (bind _values_2 (`BlueprintMapLibrary.Map_Values` (`self.CompletedQuestList`)))
  (for _array_element_2 _values_2
    (if (`KismetStringLibrary.EqualEqual_StrStr` (`/Game/DsQuestAndDialogueSystem/Blueprints/QuestSystem/BP_DSsQuestBase.GetID` _array_element_2) ID)
      (return _array_element_2)))
  (bind _values_3 (`BlueprintMapLibrary.Map_Values` (`self.FailedQuestList`)))
  (for _array_element_3 _values_3
    (if (`KismetStringLibrary.EqualEqual_StrStr` (`/Game/DsQuestAndDialogueSystem/Blueprints/QuestSystem/BP_DSsQuestBase.GetID` _array_element_3) ID)
      (return _array_element_3)))
  (return (`local.Empty`)))

(fn `GetQuestByName`
  (params (Progress :type "/Game/DsQuestAndDialogueSystem/Blueprints/Enums/Quest/Enum_DSsQuestProgression Enum" :default "NewEnumerator0") (ID :type String))
  (returns (Quest :type "/Game/DsQuestAndDialogueSystem/Blueprints/QuestSystem/BP_DSsQuestBase Object Reference"))
  (locals (Empty :type "/Game/DsQuestAndDialogueSystem/Blueprints/QuestSystem/BP_DSsQuestBase Object Reference"))
  (switch `/Game/DsQuestAndDialogueSystem/Blueprints/Enums/Quest/Enum_DSsQuestProgression` Progress
    (:`NewEnumerator0`
      (bind _values (`BlueprintMapLibrary.Map_Values` (`self.ActiveQuestList`)))
      (for _array_element _values
        (if (`KismetStringLibrary.EqualEqual_StrStr` (`/Game/DsQuestAndDialogueSystem/Blueprints/QuestSystem/BP_DSsQuestBase.GetName` _array_element) ID)
          (return _array_element)))
      (return (`local.Empty`)))
    (:`NewEnumerator1`
      (bind _values_2 (`BlueprintMapLibrary.Map_Values` (`self.CompletedQuestList`)))
      (for _array_element_2 _values_2
        (if (`KismetStringLibrary.EqualEqual_StrStr` (`/Game/DsQuestAndDialogueSystem/Blueprints/QuestSystem/BP_DSsQuestBase.GetName` _array_element_2) ID)
          (return _array_element_2)))
      (return (`local.Empty`)))
    (:`NewEnumerator2`
      (bind _values_3 (`BlueprintMapLibrary.Map_Values` (`self.FailedQuestList`)))
      (for _array_element_3 _values_3
        (if (`KismetStringLibrary.EqualEqual_StrStr` (`/Game/DsQuestAndDialogueSystem/Blueprints/QuestSystem/BP_DSsQuestBase.GetName` _array_element_3) ID)
          (return _array_element_3)))
      (return (`local.Empty`)))
    (:`NewEnumerator3`
      (return (`local.Empty`)))))

(fn `GetQuestParameter`
  (params (ID :type "/Game/DsQuestAndDialogueSystem/Blueprints/Structs/Quest/Struct_DSsQuestParameterID Structure"))
  (returns (Output :type "/Game/DsQuestAndDialogueSystem/Blueprints/QuestSystem/BP_DSsQuestParameterBase Object Reference"))
  (locals (Empty :type "/Game/DsQuestAndDialogueSystem/Blueprints/QuestSystem/BP_DSsQuestParameterBase Object Reference"))
  (bind _quest (`self.GetQuestByIDEx` ID_QuestID_10_4834D5E148B1D1234916BE874771298C))
  (bind _output (`/Game/DsQuestAndDialogueSystem/Blueprints/QuestSystem/BP_DSsQuestSectionBase.GetParameter` (`/Game/DsQuestAndDialogueSystem/Blueprints/QuestSystem/BP_DSsQuestBase.GetSection` _quest ID_SectionIndex_13_F5EAECD44347E1895BA684AA95BC1E6C) ID_Parameter_7_7BCCB6234EAE1D271D956A9CCB13BB8C))
  (`/Engine/EditorBlueprintResources/StandardMacros.IsValid` _output
    (:`Is Valid`
      (return _output))
    (:`Is Not Valid`
      (return (`local.Empty`)))))

(fn `IsQuestBlackListed`
  (params (Quest :type "/Game/DsQuestAndDialogueSystem/Blueprints/Structs/Quest/Struct_DSsQuestFramework Structure (by ref)"))
  (returns (Return :type Boolean))
  (if (`KismetArrayLibrary.Array_Contains` (`self.QuestBlackList`) Quest)
    (return true)
    (else
      (return false))))

(fn `IsQuestFailed`
  (params (Quest :type "/Game/DsQuestAndDialogueSystem/Blueprints/Structs/Quest/Struct_DSsQuestFramework Structure (by ref)"))
  (returns (NewParam :type Boolean))
  (bind _quest (`self.GetQuestByID` "NewEnumerator2" (`.QuestID_4_4DA48B5A4D4871FBE8DA14A70DAE74DD` (break `/Game/DsQuestAndDialogueSystem/Blueprints/Structs/Quest/Struct_DSsQuestFramework` Quest))))
  (`/Engine/EditorBlueprintResources/StandardMacros.IsValid` _quest
    (:`Is Valid`
      (return true))
    (:`Is Not Valid`
      (return false))))

(fn `IsQuestFailedEx`
  (params (Quest :type "DataTableRowHandle Structure (by ref)"))
  (returns (return :type Boolean))
  (bind (_datatable _rowname) (break `DataTableRowHandle` Quest))
  (bind _returnvalue (`|GetDataTableRow` _datatable _rowname)
    (:`then`
      (return (`self.IsQuestFailed` _returnvalue)))))

(fn `ParameterUpdated_Callback`
  (params (Parameter :type "/Game/DsQuestAndDialogueSystem/Blueprints/QuestSystem/BP_DSsQuestParameterBase Object Reference") (Reason :type "/Game/DsQuestAndDialogueSystem/Blueprints/Enums/Quest/Enum_DSsQuestUpdateReason Enum" :default "NewEnumerator4"))
  (`self.ParameterUpdated` Parameter Reason))

(fn `ProgressQuest`
  (params (InFragment :type "/Game/DsQuestAndDialogueSystem/Blueprints/Structs/Quest/Struct_DSsQuestFragment Structure"))
  (locals (Progressed :type Boolean))
  ;[1 1 1] Progress quest if fragment bound quest is active
  (bind _values (`BlueprintMapLibrary.Map_Values` (`self.ActiveQuestList`)))
  (for _array_element _values
    (for _array_element_2 (`.BoundToQuests_19_7512147C43A2FC7F3B0E5EAC5042E095` (break `/Game/DsQuestAndDialogueSystem/Blueprints/Structs/Quest/Struct_DSsQuestFragment` InFragment))
      (bind _returnvalue (`|GetDataTableRow` (break `DataTableRowHandle` _array_element_2) (`.RowName` (break `DataTableRowHandle` _array_element_2)))
        (:`then`
          (if (and (`KismetStringLibrary.EqualEqual_StrStr` (`.QuestID_4_4DA48B5A4D4871FBE8DA14A70DAE74DD` (break `/Game/DsQuestAndDialogueSystem/Blueprints/Structs/Quest/Struct_DSsQuestFramework` _returnvalue)) (`/Game/DsQuestAndDialogueSystem/Blueprints/QuestSystem/BP_DSsQuestBase.GetID` _array_element)) (not (`/Game/DsQuestAndDialogueSystem/Blueprints/QuestSystem/BP_DSsQuestBase.IsQuestCompleted` _array_element)) (not (`/Game/DsQuestAndDialogueSystem/Blueprints/QuestSystem/BP_DSsQuestBase.IsQuestFailed` _array_element)))
            (`/Game/DsQuestAndDialogueSystem/Blueprints/QuestSystem/BP_DSsQuestBase.Progress` _array_element InFragment)
            (`self.UpdateQuestDispatcher` _array_element "NewEnumerator13")))))))

(fn `ProgressQuestByItem`
  (params (Item :type "/Game/DsQuestAndDialogueSystem/Blueprints/FrameworkOnly/BP_DSsItemInfo Object Reference"))
  (locals (Progressed :type Boolean))
  ;[1 1 1] Progress quest if fragment bound quest is active
  (bind _values (`BlueprintMapLibrary.Map_Values` (`self.ActiveQuestList`)))
  (for _array_element _values
    (for _array_element_2 (`.BoundToQuests_19_7512147C43A2FC7F3B0E5EAC5042E095` (break `/Game/DsQuestAndDialogueSystem/Blueprints/Structs/Quest/Struct_DSsQuestFragment` (`.QuestFragment_22_94AE95B24814A21B53FA7A899A100156` (break `/Game/DsQuestAndDialogueSystem/Blueprints/Structs/Framework/Struct_DSsItemInfoBase` (`/Game/DsQuestAndDialogueSystem/Blueprints/FrameworkOnly/BP_DSsItemInfo.ItemInfo` Item)))))
      (bind _returnvalue (`|GetDataTableRow` (break `DataTableRowHandle` _array_element_2) (`.RowName` (break `DataTableRowHandle` _array_element_2)))
        (:`then`
          (if (and (`KismetStringLibrary.EqualEqual_StrStr` (`.QuestID_4_4DA48B5A4D4871FBE8DA14A70DAE74DD` (break `/Game/DsQuestAndDialogueSystem/Blueprints/Structs/Quest/Struct_DSsQuestFramework` _returnvalue)) (`/Game/DsQuestAndDialogueSystem/Blueprints/QuestSystem/BP_DSsQuestBase.GetID` _array_element)) (not (`/Game/DsQuestAndDialogueSystem/Blueprints/QuestSystem/BP_DSsQuestBase.IsQuestCompleted` _array_element)) (not (`/Game/DsQuestAndDialogueSystem/Blueprints/QuestSystem/BP_DSsQuestBase.IsQuestFailed` _array_element)))
            (`/Game/DsQuestAndDialogueSystem/Blueprints/QuestSystem/BP_DSsQuestBase.ProgressByItem` _array_element Item)
            (`self.UpdateQuestDispatcher` _array_element "NewEnumerator13")))))))

(fn `RemoveActiveQuest`
  (params (Quest :type "DataTableRowHandle Structure (by ref)"))
  (bind (_datatable _rowname) (break `DataTableRowHandle` Quest))
  (bind _activequestlist (`self.ActiveQuestList`))
  (bind _returnvalue (`|GetDataTableRow` _datatable _rowname)
    (:`then`
      (bind (_questname _questid) (break `/Game/DsQuestAndDialogueSystem/Blueprints/Structs/Quest/Struct_DSsQuestFramework` _returnvalue))
      (bind _value (`BlueprintMapLibrary.Map_Find` _activequestlist _questid))
      (`/Engine/EditorBlueprintResources/StandardMacros.IsValid` _value
        (:`Is Valid`
          (`self.RemovedQuestDispatcher` _value)
          (`BlueprintMapLibrary.Map_Remove` _activequestlist _questid))))))

(fn `RemoveFailedQuest`
  (params (Quest :type "DataTableRowHandle Structure"))
  (bind (_datatable _rowname) (break `DataTableRowHandle` Quest))
  (bind _returnvalue (`|GetDataTableRow` _datatable _rowname)
    (:`then`
      (bind (_questname _questid) (break `/Game/DsQuestAndDialogueSystem/Blueprints/Structs/Quest/Struct_DSsQuestFramework` _returnvalue))
      (bind _value (`BlueprintMapLibrary.Map_Find` (`self.FailedQuestList`) _questname))
      (`/Engine/EditorBlueprintResources/StandardMacros.IsValid` _value
        (:`Is Valid`
          (`self.RemovedQuestDispatcher` _value)
          (`BlueprintMapLibrary.Map_Remove` (`self.FailedQuestList`) _questid))))))

(fn `RemoveQuestByID`
  (params (ID :type String) (QuestStatus :type "/Game/DsQuestAndDialogueSystem/Blueprints/Enums/Quest/Enum_DSsQuestProgression Enum" :default "NewEnumerator0"))
  (bind _quest (`self.GetQuestByID` QuestStatus ID))
  (switch `/Game/DsQuestAndDialogueSystem/Blueprints/Enums/Quest/Enum_DSsQuestProgression` QuestStatus
    (:`NewEnumerator0`
      (`self.RemovedQuestDispatcher` _quest)
      (bind _id (`/Game/DsQuestAndDialogueSystem/Blueprints/QuestSystem/BP_DSsQuestBase.GetID` _quest))
      (`BlueprintMapLibrary.Map_Remove` (`self.ActiveQuestList`) _id))
    (:`NewEnumerator1`
      (`self.RemovedQuestDispatcher` _quest)
      (`BlueprintMapLibrary.Map_Remove` (`self.CompletedQuestList`) _id))
    (:`NewEnumerator2`
      (`self.RemovedQuestDispatcher` _quest)
      (`BlueprintMapLibrary.Map_Remove` (`self.FailedQuestList`) _id))))

(fn `RestartQuest`
  (params (Quest :type "/Game/DsQuestAndDialogueSystem/Blueprints/Structs/Quest/Struct_DSsQuestFramework Structure"))
  (bind (_questname _questid) (break `/Game/DsQuestAndDialogueSystem/Blueprints/Structs/Quest/Struct_DSsQuestFramework` Quest))
  (bind _quest (`self.GetQuestByIDEx` _questid))
  (`/Engine/EditorBlueprintResources/StandardMacros.IsValid` _quest
    (:`Is Valid`
      (switch `/Game/DsQuestAndDialogueSystem/Blueprints/Enums/Quest/Enum_DSsQuestProgression` (`/Game/DsQuestAndDialogueSystem/Blueprints/QuestSystem/BP_DSsQuestBase.QuestProgress` _quest)
        (:`NewEnumerator0`
          (`/Game/DsQuestAndDialogueSystem/Blueprints/QuestSystem/BP_DSsQuestBase.Restart` _quest))
        (:`NewEnumerator1`
          (`BlueprintMapLibrary.Map_Add` (`self.ActiveQuestList`) _questid _quest)
          (`BlueprintMapLibrary.Map_Remove` (`self.CompletedQuestList`) _questid)
          (`/Game/DsQuestAndDialogueSystem/Blueprints/QuestSystem/BP_DSsQuestBase.Restart` _quest))
        (:`NewEnumerator2`
          (`BlueprintMapLibrary.Map_Add` (`self.ActiveQuestList`) _questid _quest)
          (`BlueprintMapLibrary.Map_Remove` (`self.FailedQuestList`) _questid)
          (`/Game/DsQuestAndDialogueSystem/Blueprints/QuestSystem/BP_DSsQuestBase.Restart` _quest))
        (:`NewEnumerator3`
          (return))))
    (:`Is Not Valid`
      (return))))

(fn `RestartQuestEx`
  (params (Quest :type "DataTableRowHandle Structure"))
  (bind _returnvalue (`|GetDataTableRow` Quest_DataTable Quest_RowName)
    (:`then`
      (`self.RestartQuest` _returnvalue))))

(fn `RunScripts`
  (params (Scripts :type "Array of /Game/DsQuestAndDialogueSystem/Blueprints/FrameworkOnly/BP_DSsTriggerScriptBase Class Reference"))
  (for _array_element Scripts
    (bind _returnvalue (`|SpawnActorFromClass` _array_element (`KismetMathLibrary.MakeTransform` (0.0 0.0 0.0)) "Undefined" "SelectDefaultAtRuntime" null null null))
    (`/Game/DsQuestAndDialogueSystem/Blueprints/FrameworkOnly/BP_DSsTriggerScriptBase.RunScript` _returnvalue)))

(fn `ScanInventoryForNewItems_CallBack`
  (params (Quest :type "/Game/DsQuestAndDialogueSystem/Blueprints/QuestSystem/BP_DSsQuestBase Object Reference"))
  (`self.ScanInventoryForNewItems` Quest))

(fn `SectionUpdated_Callback`
  (params (Section :type "/Game/DsQuestAndDialogueSystem/Blueprints/QuestSystem/BP_DSsQuestSectionBase Object Reference") (Reason :type "/Game/DsQuestAndDialogueSystem/Blueprints/Enums/Quest/Enum_DSsQuestSectionUpdateReason Enum" :default "NewEnumerator4"))
  (`self.ParameterSectionUpdated` Section Reason))

(fn `StartQuest`
  (params (InQuest :type "DataTableRowHandle Structure"))
  (locals (ID :type String) (Temp :type "/Game/DsQuestAndDialogueSystem/Blueprints/QuestSystem/BP_DSsQuestBase Object Reference"))
  (bind (_datatable _rowname) (break `DataTableRowHandle` InQuest))
  (bind _returnvalue (`|GetDataTableRow` _datatable _rowname)
    (:`then`
      (if (not (`self.IsQuestBlackListed` _returnvalue))
        (bind _returnvalue_2 (`|GenericCreateObject` self "/Game/DsQuestAndDialogueSystem/Blueprints/QuestSystem/BP_DSsQuestBase.BP_DSsQuestBase_C" _returnvalue))
        (set `local.Temp` _returnvalue_2)
        (set `local.ID` (`/Game/DsQuestAndDialogueSystem/Blueprints/QuestSystem/BP_DSsQuestBase.GetQuestID` _returnvalue_2))
        (bind _keys (`BlueprintMapLibrary.Map_Keys` (`self.ActiveQuestList`)))
        (if (not (`KismetArrayLibrary.Array_Contains` _keys (`local.ID`)))
          (`BlueprintMapLibrary.Map_Add` (`self.ActiveQuestList`) (`local.ID`) (`local.Temp`))
          (add `/Game/DsQuestAndDialogueSystem/Blueprints/QuestSystem/BP_DSsQuestBase.ScanInventoryForNewItems` (`local.Temp`) (`|CreateDelegate` :!event `ScanInventoryForNewItems_CallBack`))
          (add `/Game/DsQuestAndDialogueSystem/Blueprints/QuestSystem/BP_DSsQuestBase.SectionUpdated` (`local.Temp`) (`|CreateDelegate` :!event `SectionUpdated_Callback`))
          (add `/Game/DsQuestAndDialogueSystem/Blueprints/QuestSystem/BP_DSsQuestBase.ParameterUpdated` (`local.Temp`) (`|CreateDelegate` :!event `ParameterUpdated_Callback`))
          (`/Game/DsQuestAndDialogueSystem/Blueprints/QuestSystem/BP_DSsQuestBase.OnCreate` (`local.Temp`))
          (`self.AddQuestDispatcher` (`local.Temp`))
          ;[1 1 1] Signal Other Quests
          (for _array_element (`.SignalOtherQuests_47_7E84C6434609FBE9249F6DB01217D9BB` (break `/Game/DsQuestAndDialogueSystem/Blueprints/Structs/Quest/Struct_DSsQuestFramework` (`/Game/DsQuestAndDialogueSystem/Blueprints/QuestSystem/BP_DSsQuestBase.QuestBase` (`local.Temp`))))
            (bind (_state _fragment) (break `/Game/DsQuestAndDialogueSystem/Blueprints/Structs/Quest/Struct_DSsQuestSignalFragment` _array_element))
            (if (`|EnumEquality` _state "NewEnumerator0")
              (`self.ProgressQuest` _fragment))))))))
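; Runtime quest object that tracks one quest's state, sections and parameters for the quest manager component, its Outer.
; OnCreate builds section objects from QuestBase data, relays their events, runs start scripts and requests an inventory scan.
; Fragments or items progress active sections, or complete or fail the quest, with optional auto-completion.
; Completion notifies the manager and runs end scripts; helpers handle restart, section chaining, lookups and reward text.
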(fn `AddParameter`
  (params (ParameterID :type "/Game/SOsQuestAndDialogueSystem/Blueprints/Structs/Quest/Struct_SOsQuestParameterID Structure") (Parameter :type "/Game/SOsQuestAndDialogueSystem/Blueprints/Structs/Quest/Struct_SOsQuestParameterBaseFramework Structure (by ref)"))
  (bind _output (`|GetArrayItem` (`self.QuestSections`) ParameterID_SectionIndex_13_F5EAECD44347E1895BA684AA95BC1E6C))
  (`/Engine/EditorBlueprintResources/StandardMacros.IsValid` _output
    (:`Is Valid`
      (`/Game/SOsQuestAndDialogueSystem/Blueprints/QuestSystem/BP_SOsQuestSectionBase.AddParameter` _output Parameter ParameterID_Parameter_7_7BCCB6234EAE1D271D956A9CCB13BB8C))))

(fn `CallNextSection`
  (params (RemovedSection :type "/Game/SOsQuestAndDialogueSystem/Blueprints/QuestSystem/BP_SOsQuestSectionBase Object Reference"))
  (bind _questsections (`self.QuestSections`))
  (bind _returnvalue (+ (`KismetArrayLibrary.Array_Find` _questsections RemovedSection) 1))
  (bind _output (`|GetArrayItem` _questsections _returnvalue))
  (if (`KismetArrayLibrary.Array_IsValidIndex` _questsections _returnvalue)
    (`/Engine/EditorBlueprintResources/StandardMacros.IsValid` _output
      (:`Is Valid`
        (if (`|EnumEquality` (`/Game/SOsQuestAndDialogueSystem/Blueprints/QuestSystem/BP_SOsQuestSectionBase.GetSectionStatus` _output) "NewEnumerator5")
          (`/Game/SOsQuestAndDialogueSystem/Blueprints/QuestSystem/BP_SOsQuestSectionBase.SetSectionStatus` _output "NewEnumerator3"))))))

(fn `CheckQuestReqCompleted`
  (returns (return :type Boolean))
  (locals (Completed :type Boolean))
  (for _array_element (`self.QuestSections`)
    (if (`/Game/SOsQuestAndDialogueSystem/Blueprints/QuestSystem/BP_SOsQuestSectionBase.CheckSectionParametersCompleted` _array_element)
      (set `local.Completed` true)
      (else
        (return false))))
  (if (`local.Completed`)
    (return (`local.Completed`))
    (else
      (return false))))

(fn `CompleteQuest`
  ;[1 1 1] If quest Active and parameters completed
  (if (and (`|EnumEquality` (`self.QuestProgress`) "NewEnumerator0") (`self.CheckQuestReqCompleted`))
    (set `self.QuestProgress` "NewEnumerator1")
    (`/Game/SOsQuestAndDialogueSystem/Blueprints/QuestSystem/BP_SOsQuestManager_Component.CompletedQuest` (`self.GetQuestManager`) self)
    (`self.RunScripts` (`.QuestEndScripts_25_7A21E4F648404E1B8E3E0197C9A754A1` (break `/Game/SOsQuestAndDialogueSystem/Blueprints/Structs/Quest/Struct_SOsQuestFramework` (`self.QuestBase`))))
    (`self.QuestUpdated` self "NewEnumerator3")
    ;[1 0 0] Determine whether recorded quest item will be removed or not. If quest item value less than current parameter value it will be consumed and removed.
    (for _array_element (`self.QuestSections`)
      (`/Game/SOsQuestAndDialogueSystem/Blueprints/QuestSystem/BP_SOsQuestSectionBase.ConsumeRecordedItems` _array_element))))

(fn `FailedQuest`
  (if (`|EnumEquality` (`self.QuestProgress`) "NewEnumerator0")
    (set `self.QuestProgress` "NewEnumerator2")
    (`/Game/SOsQuestAndDialogueSystem/Blueprints/QuestSystem/BP_SOsQuestManager_Component.FailedQuest` (`self.GetQuestManager`) self)
    (`self.QuestUpdated` self "NewEnumerator5")))

(fn `ForceCompleteQuest`
  (set `self.QuestProgress` "NewEnumerator1")
  (for _array_element (`self.QuestSections`)
    (`/Game/SOsQuestAndDialogueSystem/Blueprints/QuestSystem/BP_SOsQuestSectionBase.ForceCompleteSection` _array_element))
  (`/Game/SOsQuestAndDialogueSystem/Blueprints/QuestSystem/BP_SOsQuestManager_Component.CompletedQuest` (`self.GetQuestManager`) self)
  (`self.RunScripts` (`.QuestEndScripts_25_7A21E4F648404E1B8E3E0197C9A754A1` (break `/Game/SOsQuestAndDialogueSystem/Blueprints/Structs/Quest/Struct_SOsQuestFramework` (`self.QuestBase`))))
  (`self.QuestUpdated` self "NewEnumerator3"))

(fn `ForceFailQuest`
  (set `self.QuestProgress` "NewEnumerator2")
  (`/Game/SOsQuestAndDialogueSystem/Blueprints/QuestSystem/BP_SOsQuestManager_Component.FailedQuest` (`self.GetQuestManager`) self)
  (`self.QuestUpdated` self "NewEnumerator5"))

(fn `GetAllActiveSections`
  (returns (QuestSections :type "Array of /Game/SOsQuestAndDialogueSystem/Blueprints/QuestSystem/BP_SOsQuestSectionBase Object Reference"))
  (locals (ActiveSections :type "Array of /Game/SOsQuestAndDialogueSystem/Blueprints/QuestSystem/BP_SOsQuestSectionBase Object Reference"))
  (for _array_element (`self.QuestSections`)
    (if (`/Game/SOsQuestAndDialogueSystem/Blueprints/QuestSystem/BP_SOsQuestSectionBase.IsSectionActive` _array_element)
      (`KismetArrayLibrary.Array_Add` (`local.ActiveSections`) _array_element)))
  (return (`local.ActiveSections`)))

(fn `GetDescription`
  (returns (Description :type Text))
  (bind (_questbase_questname _questbase_questid _questbase_questdescription) (break `/Game/SOsQuestAndDialogueSystem/Blueprints/Structs/Quest/Struct_SOsQuestFramework` (`self.QuestBase`)))
  (return _questbase_questdescription))

(fn `GetID`
  (returns (ID :type String))
  (bind (_questbase_questname _questbase_questid) (break `/Game/SOsQuestAndDialogueSystem/Blueprints/Structs/Quest/Struct_SOsQuestFramework` (`self.QuestBase`)))
  (return _questbase_questid))

(fn `GetName`
  (returns (Name :type String))
  (bind _questbase_questname (break `/Game/SOsQuestAndDialogueSystem/Blueprints/Structs/Quest/Struct_SOsQuestFramework` (`self.QuestBase`)))
  (return _questbase_questname))

(fn `GetParameter`
  (params (Index :type "/Game/SOsQuestAndDialogueSystem/Blueprints/Structs/Quest/Struct_SOsQuestParameterID Structure"))
  (returns (return :type "/Game/SOsQuestAndDialogueSystem/Blueprints/QuestSystem/BP_SOsQuestParameterBase Object Reference"))
  (bind (_questid _sectionindex _parameter) (break `/Game/SOsQuestAndDialogueSystem/Blueprints/Structs/Quest/Struct_SOsQuestParameterID` Index))
  (bind _output (`|GetArrayItem` (`self.QuestSections`) _sectionindex))
  (bind _output_2 (`|GetArrayItem` (`/Game/SOsQuestAndDialogueSystem/Blueprints/QuestSystem/BP_SOsQuestSectionBase.Parameters` _output) _parameter))
  (`/Engine/EditorBlueprintResources/StandardMacros.IsValid` _output
    (:`Is Valid`
      (`/Engine/EditorBlueprintResources/StandardMacros.IsValid` _output_2
        (:`Is Valid`
          (return _output_2))))))

(fn `GetParameterByFragment`
  (params (Fragment :type "/Game/SOsQuestAndDialogueSystem/Blueprints/Structs/Quest/Struct_SOsQuestFragment Structure"))
  (returns (return :type "/Game/SOsQuestAndDialogueSystem/Blueprints/QuestSystem/BP_SOsQuestParameterBase Object Reference"))
  (for _array_element (`self.QuestSections`)
    (for _array_element_2 (`/Game/SOsQuestAndDialogueSystem/Blueprints/QuestSystem/BP_SOsQuestSectionBase.GetParameters` _array_element)
      (if (`/Game/SOsQuestAndDialogueSystem/Blueprints/QuestSystem/BP_SOsQuestParameterBase.CheckID` _array_element_2 (`.ID_7_FDF6567E4D829BC9D2B2B8968D238046` (break `/Game/SOsQuestAndDialogueSystem/Blueprints/Structs/Quest/Struct_SOsQuestFragment` Fragment)))
        (return _array_element_2)))))

(fn `GetParameterByFragmentID`
  (params (ID :type String))
  (returns (return :type "/Game/SOsQuestAndDialogueSystem/Blueprints/QuestSystem/BP_SOsQuestParameterBase Object Reference"))
  (locals (Empty :type "/Game/SOsQuestAndDialogueSystem/Blueprints/QuestSystem/BP_SOsQuestParameterBase Object Reference"))
  (for _array_element (`self.QuestSections`)
    (for _array_element_2 (`/Game/SOsQuestAndDialogueSystem/Blueprints/QuestSystem/BP_SOsQuestSectionBase.GetParameters` _array_element)
      (if (`/Game/SOsQuestAndDialogueSystem/Blueprints/QuestSystem/BP_SOsQuestParameterBase.CheckID` _array_element_2 ID)
        (return _array_element_2))))
  (return (`local.Empty`)))

(fn `GetParameterFromSection`
  (params (SectionIndex :type Integer) (ParameterIndex :type Integer))
  (returns (Output :type "/Game/SOsQuestAndDialogueSystem/Blueprints/QuestSystem/BP_SOsQuestParameterBase Object Reference"))
  (return (`/Game/SOsQuestAndDialogueSystem/Blueprints/QuestSystem/BP_SOsQuestSectionBase.GetParameter` (`|GetArrayItem` (`self.QuestSections`) SectionIndex) ParameterIndex)))

(fn `GetParameterToString`
  (params (ID :type "/Game/SOsQuestAndDialogueSystem/Blueprints/Structs/Quest/Struct_SOsQuestParameterID Structure"))
  (returns (return :type String))
  (bind (_questid _sectionindex _parameter) (break `/Game/SOsQuestAndDialogueSystem/Blueprints/Structs/Quest/Struct_SOsQuestParameterID` ID))
  (bind _output (`|GetArrayItem` (`self.QuestSections`) _sectionindex))
  (bind _output_2 (`|GetArrayItem` (`/Game/SOsQuestAndDialogueSystem/Blueprints/QuestSystem/BP_SOsQuestSectionBase.Parameters` _output) _parameter))
  (`/Engine/EditorBlueprintResources/StandardMacros.IsValid` _output
    (:`Is Valid`
      (`/Engine/EditorBlueprintResources/StandardMacros.IsValid` _output_2
        (:`Is Valid`
          (return (`/Game/SOsQuestAndDialogueSystem/Blueprints/QuestSystem/BP_SOsQuestParameterBase.ToString` _output_2)))))))

(fn `GetQuestID`
  (returns (QuestID :type String))
  (return (`.QuestID_4_4DA48B5A4D4871FBE8DA14A70DAE74DD` (break `/Game/SOsQuestAndDialogueSystem/Blueprints/Structs/Quest/Struct_SOsQuestFramework` (`self.QuestBase`)))))

(fn `GetQuestManager`
  (returns (`AsQuest Manager` :type "/Game/SOsQuestAndDialogueSystem/Blueprints/QuestSystem/BP_SOsQuestManager_Component Object Reference"))
  (return (cast `/Game/SOsQuestAndDialogueSystem/Blueprints/QuestSystem/BP_SOsQuestManager_Component` (`KismetSystemLibrary.GetOuterObject` self) :!pure true)))

(fn `GetQuestRewards`
  (returns (Rewards :type "Array of /Game/SOsQuestAndDialogueSystem/Blueprints/Structs/Quest/Struct_SOsQuestRewardFramework Structure"))
  (bind (_questbase_questname _questbase_questid _questbase_questdescription _questbase_queststartscripts _questbase_questendscripts _questbase_parametersections _questbase_rewards) (break `/Game/SOsQuestAndDialogueSystem/Blueprints/Structs/Quest/Struct_SOsQuestFramework` (`self.QuestBase`)))
  (return _questbase_rewards))

(fn `GetSection`
  (params (Index :type Integer))
  (returns (Return :type "/Game/SOsQuestAndDialogueSystem/Blueprints/QuestSystem/BP_SOsQuestSectionBase Object Reference"))
  (return (`|GetArrayItem` (`self.QuestSections`) Index)))

(fn `GetSectionByID`
  (params (ID :type String))
  (returns (Return :type "/Game/SOsQuestAndDialogueSystem/Blueprints/QuestSystem/BP_SOsQuestSectionBase Object Reference"))
  (locals (Empty :type "/Game/SOsQuestAndDialogueSystem/Blueprints/QuestSystem/BP_SOsQuestSectionBase Object Reference"))
  (for _array_element (`self.QuestSections`)
    (if (`KismetStringLibrary.EqualEqual_StrStr` (`/Game/SOsQuestAndDialogueSystem/Blueprints/QuestSystem/BP_SOsQuestSectionBase.GetID` _array_element) ID)
      (return _array_element)))
  (return (`local.Empty`)))

(fn `GetSections`
  (returns (Sections :type "Array of /Game/SOsQuestAndDialogueSystem/Blueprints/QuestSystem/BP_SOsQuestSectionBase Object Reference"))
  (return (`self.QuestSections`)))

(fn `GetSectionSize`
  (returns (return :type Integer))
  (return (`KismetArrayLibrary.Array_Length` (`self.QuestSections`))))

(fn `GetTotalParameterSize`
  (returns (return :type Integer))
  (locals (Size :type Integer :default 0))
  (for _array_element (`self.QuestSections`)
    (set `local.Size` (+ (`/Game/SOsQuestAndDialogueSystem/Blueprints/QuestSystem/BP_SOsQuestSectionBase.GetParameterSize` _array_element) (`local.Size`))))
  (return (`local.Size`)))

(fn `IsFragmentValidInput`
  (params (Fragment :type "/Game/SOsQuestAndDialogueSystem/Blueprints/Structs/Quest/Struct_SOsQuestFragment Structure"))
  (returns (Return :type Boolean))
  (`/Engine/EditorBlueprintResources/StandardMacros.IsValid` (`self.GetParameterByFragment` Fragment)
    (:`Is Valid`
      (return true))
    (:`Is Not Valid`
      (return false))))

(fn `IsQuestCompleted`
  (returns (IsQuestCompleted :type Boolean))
  (return (`|EnumEquality` (`self.QuestProgress`) "NewEnumerator1")))

(fn `IsQuestFailed`
  (returns (IsFailed :type Boolean))
  (return (`|EnumEquality` (`self.QuestProgress`) "NewEnumerator2")))

(fn `OnCreate`
  (locals (PB :type "/Game/SOsQuestAndDialogueSystem/Blueprints/QuestSystem/BP_SOsQuestParameterBase Object Reference"))
  (bind (_questname _questid _questdescription _queststartscripts _questendscripts _parametersections) (break `/Game/SOsQuestAndDialogueSystem/Blueprints/Structs/Quest/Struct_SOsQuestFramework` (`self.QuestBase`)))
  (for _array_element _parametersections
    (bind _returnvalue (`|GenericCreateObject` "/Game/SOsQuestAndDialogueSystem/Blueprints/QuestSystem/BP_SOsQuestSectionBase.BP_SOsQuestSectionBase_C" self _array_element))
    (`/Game/SOsQuestAndDialogueSystem/Blueprints/QuestSystem/BP_SOsQuestSectionBase.OnCreate` _returnvalue)
    (`KismetArrayLibrary.Array_Add` (`self.QuestSections`) _returnvalue)
    (add `/Game/SOsQuestAndDialogueSystem/Blueprints/QuestSystem/BP_SOsQuestSectionBase.ParameterUpdated` _returnvalue (`|CreateDelegate` :!event `ParameterUpdated_Callback`))
    (add `/Game/SOsQuestAndDialogueSystem/Blueprints/QuestSystem/BP_SOsQuestSectionBase.SectionUpdated` _returnvalue (`|CreateDelegate` :!event `SectionUpdated_Callback`))
    (add `self.SectionRemovedFromQuestList` (`|CreateDelegate` :!event `CallNextSection`))
    (add `/Game/SOsQuestAndDialogueSystem/Blueprints/QuestSystem/BP_SOsQuestSectionBase.ScanInventoryForNewItems` _returnvalue (`|CreateDelegate` :!event `ScanInventoryForNewItems_Callback`)))
  (`self.RunScripts` _queststartscripts)
  (`self.ScanInventoryForNewItems` self)
  (`self.QuestUpdated` self "NewEnumerator13"))

(fn `ParameterUpdated_Callback`
  (params (Parameter :type "/Game/SOsQuestAndDialogueSystem/Blueprints/QuestSystem/BP_SOsQuestParameterBase Object Reference") (Reason :type "/Game/SOsQuestAndDialogueSystem/Blueprints/Enums/Quest/Enum_SOsQuestSectionParameterUpdateReason Enum" :default "NewEnumerator4"))
  (`self.ParameterUpdated` Parameter Reason))

(fn `Progress`
  (params (Fragment :type "/Game/SOsQuestAndDialogueSystem/Blueprints/Structs/Quest/Struct_SOsQuestFragment Structure"))
  (locals (Temp :type "/Game/SOsQuestAndDialogueSystem/Blueprints/Structs/Quest/Struct_SOsQuestFragment Structure"))
  ;[1 1 1] Progress according of type of fragment. If its complete type and quest parameters is completed then quest will be completed.
  (bind _output_get (set `local.Temp` Fragment))
  (switch `/Game/SOsQuestAndDialogueSystem/Blueprints/Enums/Quest/Enum_SOsQuestFragmentStatus` (`.Type_17_AEF599254AB2E9C1B6EC91ADFF1616B3` (break `/Game/SOsQuestAndDialogueSystem/Blueprints/Structs/Quest/Struct_SOsQuestFragment` _output_get))
    (:`NewEnumerator4`
      ;[1 1 1] Progress if section active
      (for _array_element (`self.QuestSections`)
        (if (`/Game/SOsQuestAndDialogueSystem/Blueprints/QuestSystem/BP_SOsQuestSectionBase.IsSectionActive` _array_element)
          (`/Game/SOsQuestAndDialogueSystem/Blueprints/QuestSystem/BP_SOsQuestSectionBase.ProgressSection` _array_element Fragment)))
      (`self.QuestUpdated` self "NewEnumerator13")
      (if (and (`self.CheckQuestReqCompleted`) (`.AutoCompleteQuestAfterParametersCompleted_39_F078DA1149130B12982BBB815C001458` (break `/Game/SOsQuestAndDialogueSystem/Blueprints/Structs/Quest/Struct_SOsQuestFramework` (`self.QuestBase`))))
        (`self.CompleteQuest`)))
    (:`NewEnumerator0`
      (`self.CompleteQuest`))
    (:`NewEnumerator1`
      (`self.ForceCompleteQuest`))
    (:`NewEnumerator2`
      (`self.FailedQuest`))
    (:`NewEnumerator3`
      (`self.ForceFailQuest`))))

(fn `ProgressByItem`
  (params (Item :type "/Game/SOsQuestAndDialogueSystem/Blueprints/FrameworkOnly/BP_SOsItemInfo Object Reference"))
  ;[1 1 1] Progress according of type of fragment. If its complete type and quest parameters is completed then quest will be completed.
  (switch `/Game/SOsQuestAndDialogueSystem/Blueprints/Enums/Quest/Enum_SOsQuestFragmentStatus` (`.Type_17_AEF599254AB2E9C1B6EC91ADFF1616B3` (break `/Game/SOsQuestAndDialogueSystem/Blueprints/Structs/Quest/Struct_SOsQuestFragment` (`.QuestFragment_22_94AE95B24814A21B53FA7A899A100156` (break `/Game/SOsQuestAndDialogueSystem/Blueprints/Structs/Framework/Struct_SOsItemInfoBase` (`/Game/SOsQuestAndDialogueSystem/Blueprints/FrameworkOnly/BP_SOsItemInfo.ItemInfo` Item)))))
    (:`NewEnumerator4`
      ;[1 1 1] Progress if section active
      (for _array_element (`self.QuestSections`)
        (if (`/Game/SOsQuestAndDialogueSystem/Blueprints/QuestSystem/BP_SOsQuestSectionBase.IsSectionActive` _array_element)
          (`/Game/SOsQuestAndDialogueSystem/Blueprints/QuestSystem/BP_SOsQuestSectionBase.ProgressSectionByItem` _array_element Item)))
      (`self.QuestUpdated` self "NewEnumerator13")
      (if (and (`self.CheckQuestReqCompleted`) (`.AutoCompleteQuestAfterParametersCompleted_39_F078DA1149130B12982BBB815C001458` (break `/Game/SOsQuestAndDialogueSystem/Blueprints/Structs/Quest/Struct_SOsQuestFramework` (`self.QuestBase`))))
        (`self.CompleteQuest`)))
    (:`NewEnumerator0`
      (`self.CompleteQuest`))
    (:`NewEnumerator1`
      (`self.ForceCompleteQuest`))
    (:`NewEnumerator2`
      (`self.FailedQuest`))
    (:`NewEnumerator3`
      (`self.ForceFailQuest`))))

(fn `RemoveParameter`
  (params (QuestParameterID :type "/Game/SOsQuestAndDialogueSystem/Blueprints/Structs/Quest/Struct_SOsQuestParameterID Structure"))
  (bind _output (`|GetArrayItem` (`self.QuestSections`) (`.SectionIndex_13_F5EAECD44347E1895BA684AA95BC1E6C` (break `/Game/SOsQuestAndDialogueSystem/Blueprints/Structs/Quest/Struct_SOsQuestParameterID` QuestParameterID))))
  (`/Engine/EditorBlueprintResources/StandardMacros.IsValid` _output
    (:`Is Valid`
      (`/Game/SOsQuestAndDialogueSystem/Blueprints/QuestSystem/BP_SOsQuestSectionBase.RemoveParameter` _output QuestParameterID))))

(fn `Restart`
  (set `self.QuestProgress` "NewEnumerator0")
  (`KismetArrayLibrary.Array_Clear` (`self.QuestSections`))
  (`self.OnCreate`)
  (`self.QuestUpdated` self "NewEnumerator14"))

(fn `RewardsToString`
  (returns (Return :type "Array of String"))
  (locals (Strings :type "Array of String") (ItemStrings :type "Array of String") (ItemCounts :type "Array of Integer"))
  (bind _itemcounts (`local.ItemCounts`))
  (for _array_element (`.Rewards_28_BA7445934A3C4B5A80E8F88E02B2C8CC` (break `/Game/SOsQuestAndDialogueSystem/Blueprints/Structs/Quest/Struct_SOsQuestFramework` (`self.QuestBase`)))
    (bind (_type _basictype _iteminfo _fragment) (break `/Game/SOsQuestAndDialogueSystem/Blueprints/Structs/Quest/Struct_SOsQuestRewardFramework` _array_element))
    (switch `/Game/SOsQuestAndDialogueSystem/Blueprints/Enums/Quest/Enum_SOsQuestRewardType` _type
      (:`NewEnumerator0`
        (bind (_id _value) (break `/Game/SOsQuestAndDialogueSystem/Blueprints/Structs/Quest/Struct_SOsQuestRewardBasicType` _basictype))
        (`KismetArrayLibrary.Array_Add` (`local.Strings`) (`KismetStringLibrary.Concat_StrStr` _id " : " (`KismetStringLibrary.Conv_IntToString` (`KismetMathLibrary.Round` _value)))))
      (:`NewEnumerator1`
        (`KismetArrayLibrary.Array_Add` (`local.Strings`) (`KismetStringLibrary.Concat_StrStr` _id " : " (`KismetStringLibrary.Conv_DoubleToString` _value))))
      (:`NewEnumerator2`
        ;[1 1 1] Get Quest name
        (for _array_element_2 (`.BoundToQuests_19_7512147C43A2FC7F3B0E5EAC5042E095` (break `/Game/SOsQuestAndDialogueSystem/Blueprints/Structs/Quest/Struct_SOsQuestFragment` _fragment))
          (bind _returnvalue (`|GetDataTableRow` (break `DataTableRowHandle` _array_element_2) (`.RowName` (break `DataTableRowHandle` _array_element_2)))
            (:`then`
              (bind _quest (`/Game/SOsQuestAndDialogueSystem/Blueprints/QuestSystem/BP_SOsQuestManager_Component.GetQuestByID` (`self.GetQuestManager`) "NewEnumerator0" (`.QuestID_4_4DA48B5A4D4871FBE8DA14A70DAE74DD` (break `/Game/SOsQuestAndDialogueSystem/Blueprints/Structs/Quest/Struct_SOsQuestFramework` _returnvalue))))
              (`/Engine/EditorBlueprintResources/StandardMacros.IsValid` _quest
                (:`Is Valid`
                  (`KismetArrayLibrary.Array_AddUnique` (`local.Strings`) (`KismetStringLibrary.Concat_StrStr` "Updated : " (`self.GetName` _quest)))))))))
      (:`NewEnumerator3`
        (bind (_datatable _rowname) (break `DataTableRowHandle` _iteminfo))
        ;[1 1 1] Calculate item count
        (bind _returnvalue_2 (`|GetDataTableRow` _datatable _rowname)
          (:`then`
            (bind _returnvalue_3 (`KismetTextLibrary.Conv_TextToString` (`.ItemName_4_1A908DD143B9498C98FF55A1AB328CF9` (break `/Game/SOsQuestAndDialogueSystem/Blueprints/Structs/Framework/Struct_SOsItemInfoBase` _returnvalue_2))))
            (if (`KismetArrayLibrary.Array_Contains` (`local.ItemStrings`) _returnvalue_3)
              (bind _returnvalue_4 (`KismetArrayLibrary.Array_Find` (`local.ItemStrings`) _returnvalue_3))
              (`KismetArrayLibrary.Array_Set` _itemcounts _returnvalue_4 (+ 1 (`|GetArrayItem` _itemcounts _returnvalue_4)))
              (else
                (`KismetArrayLibrary.Array_AddUnique` (`local.ItemStrings`) _returnvalue_3)
                (`KismetArrayLibrary.Array_Add` (`local.ItemCounts`) 1))))))))
  (for (_array_element_3 _array_index) (`local.ItemStrings`)
    (`KismetArrayLibrary.Array_Add` (`local.Strings`) (`KismetStringLibrary.Concat_StrStr` _array_element_3 " X " (`KismetStringLibrary.Conv_IntToString` (`|GetArrayItem` (`local.ItemCounts`) _array_index)))))
  (return (`local.Strings`)))

(fn `RunScripts`
  (params (Scripts :type "Array of /Game/SOsQuestAndDialogueSystem/Blueprints/FrameworkOnly/BP_SOsTriggerScriptBase Class Reference (by ref)"))
  (`/Game/SOsQuestAndDialogueSystem/Blueprints/QuestSystem/BP_SOsQuestManager_Component.RunScripts` (`self.GetQuestManager`) Scripts))

(fn `ScanInventoryForNewItems_Callback`
  (`self.ScanInventoryForNewItems` self)
  (`self.QuestUpdated` self "NewEnumerator13"))

(fn `SectionUpdated_Callback`
  (params (Section :type "/Game/SOsQuestAndDialogueSystem/Blueprints/QuestSystem/BP_SOsQuestSectionBase Object Reference") (Reason :type "/Game/SOsQuestAndDialogueSystem/Blueprints/Enums/Quest/Enum_SOsQuestSectionUpdateReason Enum" :default "NewEnumerator4"))
  (`self.SectionUpdated` Section Reason))
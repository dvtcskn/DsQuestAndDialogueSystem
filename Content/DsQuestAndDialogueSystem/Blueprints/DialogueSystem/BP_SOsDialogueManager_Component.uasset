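; Dialogue manager component that runs branching conversations with NPCs from data table rows and tracks the current, base and visited lines.
; Options and entry dialogues are filtered by quest progress, parameter conditions and blacklists from a quest manager.
; ProgressDialogue handles jump, back, return-to-base and end types, while Tick auto-advances timed lines by set time or animation length.
; Each entered line can spawn script actors, fire rewards, and start or progress quests.
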(event `self.ReceiveTick`
  (params (DeltaSeconds :type "Float (single-precision)"))
  (bind (_options _dialogtype _timeddialogue _jumptodialog _text _conditionaltext _buttontext _rewards _questfragments _startquests _enabled _questcondition _triggerscript _animation) (break `/Game/SOsQuestAndDialogueSystem/Blueprints/Structs/Dialogue/Struct_SOsDialogueFramework` (`self.Current`)))
  (bind (_time _skippable _useanimationtimeifavailable _nextdialogue) (break `/Game/SOsQuestAndDialogueSystem/Blueprints/Structs/Dialogue/Struct_SOsTimedDialogue` _timeddialogue))
  (bind (_datatable _rowname) (break `DataTableRowHandle` _nextdialogue))
  (if (`|EnumEquality` _dialogtype "NewEnumerator8")
    (set `self.Time` (+ (`self.Time`) DeltaSeconds))
    (`/Engine/EditorBlueprintResources/StandardMacros.IsValid` _animation
      (:`Is Valid`
        (bind _returnvalue (`AnimSequenceBase.GetPlayLength` _animation)))
      (:`Is Not Valid`
        _))
    (if (>= (`self.Time`) (`KismetMathLibrary.SelectFloat` _returnvalue _time _useanimationtimeifavailable))
      (set `self.Time` 0.0)
      (bind _returnvalue_2 (`|GetDataTableRow` _datatable _rowname)
        (:`then`
          (`self.ProgressDialogue` _returnvalue_2))))
    (else
      (set `self.Time` 0.0))))

(fn `ApplyDialogueFeatures`
  (params (Dialogue :type "/Game/SOsQuestAndDialogueSystem/Blueprints/Structs/Dialogue/Struct_SOsDialogueFramework Structure (by ref)"))
  (bind (_options _dialogtype _timeddialogue _jumptodialog _text _conditionaltext _buttontext _rewards _questfragments _startquests _enabled _questcondition _triggerscript) (break `/Game/SOsQuestAndDialogueSystem/Blueprints/Structs/Dialogue/Struct_SOsDialogueFramework` Dialogue))
  (`self.RunScriptsFromDialogue` _triggerscript)
  (`self.DialogueRewards` Dialogue)
  (for _array_element _startquests
    (bind (_datatable _rowname) (break `DataTableRowHandle` _array_element))
    (`/Game/SOsQuestAndDialogueSystem/Blueprints/QuestSystem/BP_SOsQuestManager_Component.StartQuest` (`self.GetQuestManager`) (make `DataTableRowHandle` _datatable _rowname)))
  (for _array_element_2 _questfragments
    (`/Game/SOsQuestAndDialogueSystem/Blueprints/QuestSystem/BP_SOsQuestManager_Component.ProgressQuest` (`self.GetQuestManager`) _array_element_2)))

(fn `EndCoversation`
  (locals (Empty :type "Actor Object Reference"))
  (set `self.DialogueOwner` (`local.Empty`))
  (set `self.ConversationStatus` false)
  (`KismetArrayLibrary.Array_Clear` (`self.VisitedDialogOptions`))
  (`KismetArrayLibrary.Array_Clear` (`self.FilteredDialogOptions`))
  (`self.CoversationEnded` (`self.DialogueOwner`)))

(fn `EnterDialogue`
  (params (Dialogue :type "/Game/SOsQuestAndDialogueSystem/Blueprints/Structs/Dialogue/Struct_SOsDialogueFramework Structure"))
  (locals (Empty :type "Actor Object Reference"))
  ;[1 1 1] Check if dialog is active
  (if (`self.IsItActive` Dialogue (`self.GetQuestManager`))
    (bind _output_get (set `self.Current` Dialogue))
    (set `self.Base` _output_get)
    (set `self.ConversationStatus` true)
    (`self.FilterCurrentDialogueOptions`)
    (`self.ApplyDialogueFeatures` (`self.Current`))
    (`self.CoversationStarted` (`local.Empty`))))

(fn `EnterDialogueEx`
  (params (Dialogue :type "DataTableRowHandle Structure"))
  (bind _returnvalue (`|GetDataTableRow` Dialogue_DataTable Dialogue_RowName)
    (:`then`
      (`self.EnterDialogue` _returnvalue))))

(fn `EnterDialogueWithNPC`
  (params (NPC :type "Character Object Reference") (Dialogue :type "/Game/SOsQuestAndDialogueSystem/Blueprints/Structs/Dialogue/Struct_SOsDialogueFramework Structure"))
  ;[1 1 1] Check if dialog is active
  (if (`self.IsItActive` Dialogue (`self.GetQuestManager`))
    (bind _output_get (set `self.Current` Dialogue))
    (set `self.Base` _output_get)
    (set `self.ConversationStatus` true)
    (set `self.DialogueOwner` NPC)
    (`self.FilterCurrentDialogueOptions`)
    (`self.ApplyDialogueFeatures` (`self.Current`))
    (`self.CoversationStarted` (`self.DialogueOwner`))))

(fn `EnterDialogueWithNPCEx`
  (params (NPC :type "Character Object Reference") (Dialogue :type "DataTableRowHandle Structure"))
  (bind _returnvalue (`|GetDataTableRow` Dialogue_DataTable Dialogue_RowName)
    (:`then`
      (`self.EnterDialogueWithNPC` NPC _returnvalue))))

(fn `FilterCurrentDialogueOptions`
  (set `self.FilteredDialogOptions` (`self.FilterCurrentOptions` (`self.GetQuestManager`))))

(fn `FilterCurrentOptions`
  (params (QuestManager :type "/Game/SOsQuestAndDialogueSystem/Blueprints/QuestSystem/BP_SOsQuestManager_Component Object Reference"))
  (returns (ConversationOptions :type "Array of DataTableRowHandle Structure"))
  (locals (Banned :type Boolean) (TableData :type "Array of DataTableRowHandle Structure"))
  (for _array_element (`.Options_71_C02332094F03F85A9EE7ACA39B32546A` (break `/Game/SOsQuestAndDialogueSystem/Blueprints/Structs/Dialogue/Struct_SOsDialogueFramework` (`self.Current`)))
    (bind (_datatable _rowname) (break `DataTableRowHandle` _array_element))
    (bind _returnvalue (`|GetDataTableRow` _datatable _rowname)
      (:`then`
        (bind (_options _dialogtype _timeddialogue _jumptodialog _text _conditionaltext _buttontext _rewards _questfragments _startquests _enabled _questcondition) (break `/Game/SOsQuestAndDialogueSystem/Blueprints/Structs/Dialogue/Struct_SOsDialogueFramework` _returnvalue))
        ;[1 0 0] Quest condition check
        (if (not (== (`KismetArrayLibrary.Array_Length` _questcondition) 0))
          (set `local.Banned` false)
          (for _array_element_2 _questcondition
            (if (not (`local.Banned`))
              (bind (_quest _questprogress _questparameterconditions) (break `/Game/SOsQuestAndDialogueSystem/Blueprints/Structs/Dialogue/Struct_SOsDialogueQuestProgressCondition` _array_element_2))
              (bind (_datatable_2 _rowname_2) (break `DataTableRowHandle` _quest))
              (bind _returnvalue_2 (`|GetDataTableRow` _datatable_2 _rowname_2)
                (:`then`
                  (bind _quest_2 (`/Game/SOsQuestAndDialogueSystem/Blueprints/QuestSystem/BP_SOsQuestManager_Component.GetQuestByIDEx` QuestManager (`.QuestID_4_4DA48B5A4D4871FBE8DA14A70DAE74DD` (break `/Game/SOsQuestAndDialogueSystem/Blueprints/Structs/Quest/Struct_SOsQuestFramework` _returnvalue_2))))
                  (`/Engine/EditorBlueprintResources/StandardMacros.IsValid` _quest_2
                    (:`Is Valid`
                      (switch `/Game/SOsQuestAndDialogueSystem/Blueprints/Enums/Dialogue/Enum_SOsDialogueQuestProgressCondition` _questprogress
                        (:`NewEnumerator8`
                          (set `local.Banned` true))
                        (:`NewEnumerator9`
                          (bind _questprogress_2 (`/Game/SOsQuestAndDialogueSystem/Blueprints/QuestSystem/BP_SOsQuestBase.QuestProgress` _quest_2))
                          (if (`|EnumEquality` _questprogress_2 "NewEnumerator0")
                            (if (> (`KismetArrayLibrary.Array_Length` _questparameterconditions) 0) :!label _label
                              ;[1 0 0] Quest parameter condition check
                              (for _array_element_3 _questparameterconditions
                                (bind (_sectionindex _parameterindex _enabled_2 _completed) (break `/Game/SOsQuestAndDialogueSystem/Blueprints/Structs/Dialogue/Struct_SOsDialogueQuestParameterProgressCondition` _array_element_3))
                                (if (<= (+ _parameterindex 1) (`/Game/SOsQuestAndDialogueSystem/Blueprints/QuestSystem/BP_SOsQuestSectionBase.GetParameterSize` (`/Game/SOsQuestAndDialogueSystem/Blueprints/QuestSystem/BP_SOsQuestBase.GetSection` _quest_2 _sectionindex)))
                                  (bind _output (`/Game/SOsQuestAndDialogueSystem/Blueprints/QuestSystem/BP_SOsQuestBase.GetParameterFromSection` _quest_2 _sectionindex _parameterindex))
                                  (if (== (`/Game/SOsQuestAndDialogueSystem/Blueprints/QuestSystem/BP_SOsQuestParameterBase.IsEnabled` _output) _enabled_2)
                                    (if (== (`/Game/SOsQuestAndDialogueSystem/Blueprints/QuestSystem/BP_SOsQuestParameterBase.GetIsCompleted` _output) _completed)
                                      (set `local.Banned` false)
                                      (else
                                        (set `local.Banned` true)))
                                    (else
                                      (set `local.Banned` true)))
                                  (else
                                    (set `local.Banned` true)))))
                            (else
                              (set `local.Banned` true :!label _label_2))))
                        (:`NewEnumerator10`
                          (if (`|EnumEquality` _questprogress_2 "NewEnumerator1")
                            (goto _label)
                            (else
                              (goto _label_2))))
                        (:`NewEnumerator11`
                          (if (`|EnumEquality` _questprogress_2 "NewEnumerator2")
                            (goto _label)
                            (else
                              (goto _label_2))))
                        (:`NewEnumerator12`
                          (if (`|EnumInequality` _questprogress_2 "NewEnumerator2")
                            (if (`/Game/SOsQuestAndDialogueSystem/Blueprints/QuestSystem/BP_SOsQuestManager_Component.IsQuestBlackListed` QuestManager _returnvalue_2) :!label _label_3
                              (set `local.Banned` true)
                              (else
                                (goto _label)))
                            (else
                              (goto _label_2))))
                        (:`NewEnumerator13`
                          (if (`|EnumInequality` _questprogress_2 "NewEnumerator1")
                            (goto _label)
                            (else
                              (goto _label_2))))
                        (:`NewEnumerator14`
                          (if (and (`|EnumInequality` _questprogress_2 "NewEnumerator2") (`|EnumInequality` _questprogress_2 "NewEnumerator1"))
                            (goto _label_3)
                            (else
                              (goto _label_2))))))
                    (:`Is Not Valid`
                      (if (or (`|EnumEquality` _questprogress "NewEnumerator8") (`|EnumEquality` _questprogress "NewEnumerator12") (`|EnumEquality` _questprogress "NewEnumerator13") (`|EnumEquality` _questprogress "NewEnumerator14"))
                        (if (`/Game/SOsQuestAndDialogueSystem/Blueprints/QuestSystem/BP_SOsQuestManager_Component.IsQuestBlackListed` QuestManager _returnvalue_2)
                          (set `local.Banned` true)
                          (else
                            (set `local.Banned` false)))
                        (else
                          (set `local.Banned` true)))))))))
          ;;[0 0 0] if Dialog option accessible(not banned), add to the list
          (if (not (`local.Banned`))
            (`KismetArrayLibrary.Array_Add` (`local.TableData`) _array_element))
          (else
            (`KismetArrayLibrary.Array_Add` (`local.TableData`) _array_element))))))
  (return (`local.TableData`)))

(fn `GetCurrentDialogueFilteredOptions`
  (returns (Options :type "Array of DataTableRowHandle Structure"))
  (return (`self.FilteredDialogOptions`)))

(fn `GetCurrentDialogueText`
  (returns (Return :type Text))
  (locals (LocalText :type Text))
  (bind _options (`self.GetCurrentDialogueFilteredOptions`))
  (bind (_options_2 _dialogtype _timeddialogue _jumptodialog _text _conditionaltext) (break `/Game/SOsQuestAndDialogueSystem/Blueprints/Structs/Dialogue/Struct_SOsDialogueFramework` (`self.Current`)))
  (set `local.LocalText` _text)
  (if (not (> (`BlueprintMapLibrary.Map_Length` _conditionaltext) 0))
    (return (`local.LocalText`))
    (else
      (bind _values (`BlueprintMapLibrary.Map_Values` _conditionaltext))
      (for _array_element _values
        (bind _keys (`BlueprintMapLibrary.Map_Keys` _conditionaltext))
        (bind _output (`|GetArrayItem` (`.Options_71_C02332094F03F85A9EE7ACA39B32546A` (break `/Game/SOsQuestAndDialogueSystem/Blueprints/Structs/Dialogue/Struct_SOsDialogueFramework` (`self.Current`))) _array_element))
        (bind (_datatable _rowname) (break `DataTableRowHandle` _output))
        (bind (_datatable_2 _rowname_2) (break `DataTableRowHandle` (`|GetArrayItem` _options (`KismetArrayLibrary.Array_Find` _options _output))))
        (if (and (== _datatable _datatable_2) (== _rowname _rowname_2))
          (set `local.LocalText` (`KismetTextLibrary.Conv_StringToText` (`|GetArrayItem` _keys _array_element)))))
      (return (`local.LocalText`)))))

(fn `GetDialogueOwner`
  (returns (Return :type "Actor Object Reference"))
  (return (`self.DialogueOwner`)))

(fn `GetQuestManager`
  (returns (Return :type "/Game/SOsQuestAndDialogueSystem/Blueprints/QuestSystem/BP_SOsQuestManager_Component Object Reference"))
  (return (`self.QuestManager`)))

(fn `IsCurrentDialogueFilteredOptionsAvailable`
  (returns (ReturnValue :type Boolean))
  (return (> (`KismetArrayLibrary.Array_Length` (`self.FilteredDialogOptions`)) 0)))

(fn `IsItActive`
  (params (Dialogue :type "/Game/SOsQuestAndDialogueSystem/Blueprints/Structs/Dialogue/Struct_SOsDialogueFramework Structure") (QuestManager :type "/Game/SOsQuestAndDialogueSystem/Blueprints/QuestSystem/BP_SOsQuestManager_Component Object Reference"))
  (returns (Return :type Boolean))
  (locals (Banned :type Boolean))
  ;[0 0 0] Quest Condition Check
  (for _array_element (`.QuestCondition_90_91D16C474A4D8624782EFFB5A9CD27C3` (break `/Game/SOsQuestAndDialogueSystem/Blueprints/Structs/Dialogue/Struct_SOsDialogueFramework` Dialogue))
    (bind (_quest _questprogress _questparameterconditions) (break `/Game/SOsQuestAndDialogueSystem/Blueprints/Structs/Dialogue/Struct_SOsDialogueQuestProgressCondition` _array_element))
    (bind (_datatable _rowname) (break `DataTableRowHandle` _quest))
    (bind _returnvalue (`|GetDataTableRow` _datatable _rowname)
      (:`then`
        (bind _quest_2 (`/Game/SOsQuestAndDialogueSystem/Blueprints/QuestSystem/BP_SOsQuestManager_Component.GetQuestByIDEx` QuestManager (`.QuestID_4_4DA48B5A4D4871FBE8DA14A70DAE74DD` (break `/Game/SOsQuestAndDialogueSystem/Blueprints/Structs/Quest/Struct_SOsQuestFramework` _returnvalue))))
        (`/Engine/EditorBlueprintResources/StandardMacros.IsValid` _quest_2
          (:`Is Valid`
            (switch `/Game/SOsQuestAndDialogueSystem/Blueprints/Enums/Dialogue/Enum_SOsDialogueQuestProgressCondition` _questprogress
              (:`NewEnumerator8`
                (set `local.Banned` true))
              (:`NewEnumerator9`
                (bind _questprogress_2 (`/Game/SOsQuestAndDialogueSystem/Blueprints/QuestSystem/BP_SOsQuestBase.QuestProgress` _quest_2))
                (if (`|EnumEquality` _questprogress_2 "NewEnumerator0")
                  (if (> (`KismetArrayLibrary.Array_Length` _questparameterconditions) 0) :!label _label
                    ;[0 0 0] Quest Parameter Condition Check
                    (for _array_element_2 _questparameterconditions
                      (bind (_sectionindex _parameterindex _enabled _completed) (break `/Game/SOsQuestAndDialogueSystem/Blueprints/Structs/Dialogue/Struct_SOsDialogueQuestParameterProgressCondition` _array_element_2))
                      (if (<= (+ _parameterindex 1) (`/Game/SOsQuestAndDialogueSystem/Blueprints/QuestSystem/BP_SOsQuestSectionBase.GetParameterSize` (`/Game/SOsQuestAndDialogueSystem/Blueprints/QuestSystem/BP_SOsQuestBase.GetSection` _quest_2 _sectionindex)))
                        (bind _output (`/Game/SOsQuestAndDialogueSystem/Blueprints/QuestSystem/BP_SOsQuestBase.GetParameterFromSection` _quest_2 _sectionindex _parameterindex))
                        (if (== (`/Game/SOsQuestAndDialogueSystem/Blueprints/QuestSystem/BP_SOsQuestParameterBase.IsEnabled` _output) _enabled)
                          (if (== (`/Game/SOsQuestAndDialogueSystem/Blueprints/QuestSystem/BP_SOsQuestParameterBase.GetIsCompleted` _output) _completed)
                            (set `local.Banned` false)
                            (else
                              (set `local.Banned` true)))
                          (else
                            (set `local.Banned` true)))
                        (else
                          (set `local.Banned` true)))))
                  (else
                    (set `local.Banned` true :!label _label_2))))
              (:`NewEnumerator10`
                (if (`|EnumEquality` _questprogress_2 "NewEnumerator1")
                  (goto _label)
                  (else
                    (goto _label_2))))
              (:`NewEnumerator11`
                (if (`|EnumEquality` _questprogress_2 "NewEnumerator2")
                  (goto _label)
                  (else
                    (goto _label_2))))
              (:`NewEnumerator12`
                (if (`|EnumInequality` _questprogress_2 "NewEnumerator2")
                  (if (`/Game/SOsQuestAndDialogueSystem/Blueprints/QuestSystem/BP_SOsQuestManager_Component.IsQuestBlackListed` QuestManager _returnvalue) :!label _label_3
                    (set `local.Banned` true)
                    (else
                      (goto _label)))
                  (else
                    (goto _label_2))))
              (:`NewEnumerator13`
                (if (`|EnumInequality` _questprogress_2 "NewEnumerator1")
                  (goto _label)
                  (else
                    (goto _label_2))))
              (:`NewEnumerator14`
                (if (and (`|EnumInequality` _questprogress_2 "NewEnumerator2") (`|EnumInequality` _questprogress_2 "NewEnumerator1"))
                  (goto _label_3)
                  (else
                    (goto _label_2))))))
          (:`Is Not Valid`
            (if (or (`|EnumEquality` _questprogress "NewEnumerator8") (`|EnumEquality` _questprogress "NewEnumerator12") (`|EnumEquality` _questprogress "NewEnumerator13") (`|EnumEquality` _questprogress "NewEnumerator14"))
              (if (`/Game/SOsQuestAndDialogueSystem/Blueprints/QuestSystem/BP_SOsQuestManager_Component.IsQuestBlackListed` QuestManager _returnvalue)
                (set `local.Banned` true)
                (else
                  (set `local.Banned` false)))
              (else
                (set `local.Banned` true))))))))
  (return (not (`local.Banned`))))

(fn `IsItInConversation`
  (returns (Return :type Boolean))
  (return (`self.ConversationStatus`)))

(fn `ProgressDialogue`
  (params (Dialogue :type "/Game/SOsQuestAndDialogueSystem/Blueprints/Structs/Dialogue/Struct_SOsDialogueFramework Structure"))
  (bind (_options _dialogtype _timeddialogue _jumptodialog _text) (break `/Game/SOsQuestAndDialogueSystem/Blueprints/Structs/Dialogue/Struct_SOsDialogueFramework` Dialogue))
  (bind _visiteddialogoptions (`self.VisitedDialogOptions`))
  (bind (_datatable _rowname) (break `DataTableRowHandle` _jumptodialog))
  (bind (_datatable_2 _rowname_2) (break `DataTableRowHandle` _jumptodialog))
  (bind _returnvalue (- (`KismetArrayLibrary.Array_Length` _visiteddialogoptions) 3))
  ;[1 0 0] After the option is selected, filter the options of the Selected option, then proceed according to the type of the selected option.
  (if (not (`self.IsCurrentDialogueFilteredOptionsAvailable`))
    (`self.FilterCurrentDialogueOptions`))
  (`KismetArrayLibrary.Array_Add` (`self.VisitedDialogOptions`) Dialogue)
  (`self.ApplyDialogueFeatures` Dialogue)
  (if (`|EnumEquality` _dialogtype "NewEnumerator6")
    (set `self.Current` (`self.Base`))
    (`self.FilterCurrentDialogueOptions`)
    (`self.OnCoversationProgress` (`self.DialogueOwner`) (`self.Current`))
    (elif (and (`|EnumEquality` _dialogtype "NewEnumerator7") (`KismetArrayLibrary.Array_IsValidIndex` _visiteddialogoptions _returnvalue))
      (bind _output_get (set `self.Current` (`|GetArrayItem` (`self.VisitedDialogOptions`) _returnvalue)))
      (`KismetArrayLibrary.Array_Add` (`self.VisitedDialogOptions`) _output_get)
      (`self.FilterCurrentDialogueOptions`)
      (`self.OnCoversationProgress` (`self.DialogueOwner`) (`self.Current`))
      (elif (and (`|EnumInequality` _dialogtype "NewEnumerator4") (`|EnumInequality` _dialogtype "NewEnumerator2") (`|EnumInequality` _dialogtype "NewEnumerator5"))
        (set `self.Current` Dialogue)
        (`self.FilterCurrentDialogueOptions`)
        (`self.OnCoversationProgress` (`self.DialogueOwner`) (`self.Current`))
        (elif (`|EnumEquality` _dialogtype "NewEnumerator2")
          (bind _returnvalue_2 (`|GetDataTableRow` _datatable_2 _rowname_2)
            (:`then`
              (set `self.Current` _returnvalue_2)
              (`self.FilterCurrentDialogueOptions`)
              (`self.OnCoversationProgress` (`self.DialogueOwner`) (`self.Current`))))
          (elif (`|EnumEquality` _dialogtype "NewEnumerator5")
            (bind _returnvalue_3 (`|GetDataTableRow` _datatable _rowname)
              (:`then`
                (bind _output_get_2 (set `self.Current` _returnvalue_3))
                (setmembers `/Game/SOsQuestAndDialogueSystem/Blueprints/Structs/Dialogue/Struct_SOsDialogueFramework` :`StructRef` _output_get_2 :`Text` _text)
                (`self.FilterCurrentDialogueOptions`)
                (`self.OnCoversationProgress` (`self.DialogueOwner`) (`self.Current`))))
            (elif (`|EnumEquality` _dialogtype "NewEnumerator4")
              (`self.EndCoversation`))))))))

(fn `RunScriptsFromDialogue`
  (params (Script :type "Array of /Game/SOsQuestAndDialogueSystem/Blueprints/FrameworkOnly/BP_SOsTriggerScriptBase Class Reference"))
  (for _array_element Script
    (`|SpawnActorFromClass` _array_element (`KismetMathLibrary.MakeTransform` (0.0 0.0 0.0)) "AdjustIfPossibleButAlwaysSpawn" "OverrideRootScale" null (`self.DialogueOwner`) null)))

(fn `SetQuestManager`
  (params (QuestManager :type "/Game/SOsQuestAndDialogueSystem/Blueprints/QuestSystem/BP_SOsQuestManager_Component Object Reference"))
  (set `self.QuestManager` QuestManager))

(fn `SkipActiveTimedDialogue`
  (bind (_options _dialogtype _timeddialogue) (break `/Game/SOsQuestAndDialogueSystem/Blueprints/Structs/Dialogue/Struct_SOsDialogueFramework` (`self.Current`)))
  (bind (_time _skippable _useanimationtimeifavailable _nextdialogue) (break `/Game/SOsQuestAndDialogueSystem/Blueprints/Structs/Dialogue/Struct_SOsTimedDialogue` _timeddialogue))
  (bind (_datatable _rowname) (break `DataTableRowHandle` _nextdialogue))
  (if (and (`|EnumEquality` _dialogtype "NewEnumerator8") _skippable)
    (set `self.Time` 0.0)
    (bind _returnvalue (`|GetDataTableRow` _datatable _rowname)
      (:`then`
        (`self.ProgressDialogue` _returnvalue)
        (`self.OnSkipTimedDialogue` (`self.DialogueOwner`) (`self.Current`))))))